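; Blueprint function library of shared gameplay helpers for the game's stats, accessories and global access.
; Math helpers scale amounts by percentage multipliers, add accessory attribute structs field by field, and pick an index from cumulative integer weights.
; Accessors reach the player character, resource manager and player data through GameMode or GI_Undeader, and forward AddPP to the level manager.
; Accessory lookup scans AccDataTable rows for a matching AccName.
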(fn `Add Acc Attribute`
  (params (Target :type "/Game/Blueprints/Accessorys/AdditionalAttribute Structure (by ref)") (Add :type "/Game/Blueprints/Accessorys/AdditionalAttribute Structure (by ref)"))
  (returns (StructOut :type "/Game/Blueprints/Accessorys/AdditionalAttribute Structure (by ref)"))
  (bind (_damagemult _attackspeedadd _clipadd _critdamagemult _critpercentadd _golddroppercentadd _expearnpercentadd _healperkilladd _healonstageclear _maxhealthadd _staminarecoverdelayreduce) (break `/Game/Blueprints/Accessorys/AdditionalAttribute` Add))
  (bind (_damagemult_2 _attackspeedadd_2 _clipadd_2 _critdamagemult_2 _critpercentadd_2 _golddroppercentadd_2 _expearnpercentadd_2 _healperkilladd_2 _healonstageclear_2 _maxhealthadd_2 _staminarecoverdelayreduce_2) (break `/Game/Blueprints/Accessorys/AdditionalAttribute` Target))
  (bind _structout (setmembers `/Game/Blueprints/Accessorys/AdditionalAttribute` :`StructRef` Target :`DamageMult` (+ _damagemult_2 _damagemult) :`AttackSpeedAdd` (+ _attackspeedadd_2 _attackspeedadd) :`ClipAdd` (+ _clipadd_2 _clipadd) :`CritDamageMult` (+ _critdamagemult_2 _critdamagemult) :`CritPercentAdd` (+ _critpercentadd_2 _critpercentadd) :`GoldDropPercentAdd` (+ _golddroppercentadd_2 _golddroppercentadd) :`ExpEarnPercentAdd` (+ _expearnpercentadd_2 _expearnpercentadd) :`HealPerKillAdd` (+ _healperkilladd_2 _healperkilladd) :`HealOnStageClear` (+ _healonstageclear_2 _healonstageclear) :`MaxHealthAdd` (+ _maxhealthadd_2 _maxhealthadd) :`StaminaRecoverDelayReduce` (+ _staminarecoverdelayreduce_2 _staminarecoverdelayreduce)))
  (return _structout))

(fn `Add PP Global`
  (params (m_Target :type "Actor Object Reference"))
  (bind _asbp_third_person_game_mode (cast `/Game/Blueprints/BP_ThirdPersonGameMode` (`GameplayStatics.GetGameMode` m_Target)))
  (`/Game/Blueprints/Level/BP_LevelManager.AddPP` (`/Game/Blueprints/BP_ThirdPersonGameMode.BP_LevelManager` _asbp_third_person_game_mode) m_Target))

(fn `Find Acc Data by Name`
  (params (accName :type Name))
  (returns (foundData :type "/Game/Blueprints/DataStructure/AccData Structure"))
  (locals (m_accName :type Name) (`found data` :type "/Game/Blueprints/DataStructure/AccData Structure"))
  (set `local.m_accName` accName)
  (bind _outrownames (`DataTableFunctionLibrary.GetDataTableRowNames` "/Game/Blueprints/DataStructure/AccDataTable.AccDataTable"))
  (for _array_element _outrownames
    (bind _returnvalue (`|GetDataTableRow` "/Game/Blueprints/DataStructure/AccDataTable.AccDataTable" _array_element)
      (:`then`
        (if (== (`local.m_accName`) (`.AccName_25_3F12C9F04EC0BB39E9EDDA99E5906E65` (break `/Game/Blueprints/DataStructure/AccData` _returnvalue)))
          (return _returnvalue))))))

(fn `Get Idx by Int Arr`
  (params (NewParam :type "Array of Integer"))
  (returns (`Array Index` :type Integer))
  (locals (Rand :type Integer :default 0) (Sum :type Integer))
  (set `local.Rand` (`KismetMathLibrary.RandomIntegerInRange` 0 100))
  (for (_array_element _array_index) NewParam
    (bind _output_get (set `local.Sum` (+ (`local.Sum`) _array_element)))
    (if (< (`local.Rand`) _output_get)
      (return _array_index))))

(fn `Get Mult Adjusted (decrease)`
  (params (Amout :type "Float (double-precision)") (Mult :type "Float (double-precision)"))
  (returns (output :type "Float (double-precision)"))
  (return (* Amout (/ 100.0 (+ Mult 100.0)))))

(fn `Get Mult Adjusted (increase)`
  (params (Amout :type "Float (double-precision)") (Mult :type "Float (double-precision)"))
  (returns (output :type "Float (double-precision)"))
  (return (* Amout (/ (+ Mult 100.0) 100.0))))

(fn `GetBP_PlayerCharacter`
  (params (WorldContextObject :type "Object Object Reference"))
  (returns (BP_PlayerCharacter :type "/Game/Blueprints/PlayerCharacter/BP_PlayerCharacter Object Reference"))
  (bind _asbp_third_person_game_mode (cast `/Game/Blueprints/BP_ThirdPersonGameMode` (`GameplayStatics.GetGameMode` WorldContextObject)))
  (bind _bp_playercharacter (`/Game/Blueprints/BP_ThirdPersonGameMode.GetBP_PlayerCharacter` _asbp_third_person_game_mode))
  (return _bp_playercharacter))

(fn `GetBP_ResManager`
  (params (WorldContextObject :type "Object Object Reference"))
  (returns (BP_PlayerResManager :type "/Game/Blueprints/PlayerRes/BP_PlayerResManager Object Reference"))
  (bind _asbp_third_person_game_mode (cast `/Game/Blueprints/BP_ThirdPersonGameMode` (`GameplayStatics.GetGameMode` WorldContextObject)))
  (return (`/Game/Blueprints/BP_ThirdPersonGameMode.BP_PlayerResManager` _asbp_third_person_game_mode)))

(fn `GetPlayerData`
  (params (WorldContextObject :type "Object Object Reference"))
  (returns (PlayerData :type "/Game/Blueprints/PlayerData Structure"))
  (bind _asgi_undeader (cast `/Game/Blueprints/GI_Undeader` (`GameplayStatics.GetGameInstance` WorldContextObject)))
  (return (`/Game/Blueprints/GI_Undeader.PlayerData` _asgi_undeader)))

(fn `Mult Acc Attribute`
  (params (Target :type "/Game/Blueprints/Accessorys/AdditionalAttribute Structure (by ref)") (mult :type Integer))
  (returns (StructOut :type "/Game/Blueprints/Accessorys/AdditionalAttribute Structure (by ref)"))
  (locals (_Target :type "/Game/Blueprints/Accessorys/AdditionalAttribute Structure"))
  (bind __target (`local._Target`))
  (set `local._Target` Target)
  (for _ (range 1 (+ mult 1))
    (bind _structout (`self.Add Acc Attribute` __target __target))
    (bind _output_get (set `local._Target` _structout))
    (return _output_get)))

(fn `SetPlayerData`
  (params (PlayerData :type "/Game/Blueprints/PlayerData Structure"))
  (bind _asgi_undeader (cast `/Game/Blueprints/GI_Undeader` (`GameplayStatics.GetGameInstance` null)))
  (set `/Game/Blueprints/GI_Undeader.PlayerData` PlayerData _asgi_undeader))