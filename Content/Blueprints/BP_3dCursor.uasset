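; BP_3dCursor is an actor that follows the mouse cursor in the 3D world.
; Each Tick it deprojects the mouse position and runs a complex multi line trace along that ray on a custom trace channel.
; It teleports to the first hit lying below a small height margin above the bottom of the player character's colliding bounds, skipping higher hits.
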(event `self.ReceiveTick`
  (params (DeltaSeconds :type "Float (single-precision)"))
  (bind _returnvalue (`GameplayStatics.GetPlayerController` 0))
  (bind (_origin _boxextent) (`self.GetActorBounds` (`GameplayStatics.GetPlayerCharacter` 0) true false))
  (bind (_locationx _locationy) (`PlayerController.GetMousePosition` _returnvalue))
  (bind (_worldposition _worlddirection) (`GameplayStatics.DeprojectScreenToWorld` _returnvalue (`KismetMathLibrary.MakeVector2D` _locationx _locationy)))
  (bind _outhits (`KismetSystemLibrary.LineTraceMulti` _worldposition (+ _worldposition (* _worlddirection 10000.0)) "TraceTypeQuery5" true))
  (for _array_element _outhits
    (bind (_bblockinghit _binitialoverlap _time _distance _location) (`GameplayStatics.BreakHitResult` _array_element))
    (if (> (+ (.z (- _origin _boxextent)) 50.0) (.z _location))
      (`self.K2_SetActorLocation` _location false true)
      (break))))

(fn `UserConstructionScript`)