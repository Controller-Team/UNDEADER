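; Health component that tracks current and maximum health and broadcasts init, increase, decrease and death events through dispatchers.
; Flat or percent-of-max adjustments are clamped between zero and max, with a death check on non-positive changes.
; Clamping goes through SetCurrHealth, so every adjustment also fires the init dispatcher.
; MultMaxHealth rescales max from the starting value and heals by any increase, but does not re-clamp current health on a decrease.
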(event `SetCurrHealth`
  (params (CurrHealth :type Integer))
  (set `self.CurrHealth` CurrHealth)
  (`self.OnInitEventDispatcher`))

(event `InitHealthSystem`
  (bind _output_get (set `self.MaxHealth` (`self.StartMaxHealth`)))
  (set `self.CurrHealth` _output_get)
  (`self.OnInitEventDispatcher`))

(event `AdjustHealth`
  (params (adjust :type Integer))
  (set `self.CurrHealth` (+ adjust (`self.CurrHealth`)))
  (`self.UpdateCurrHealthInMax`)
  (if (> adjust 0)
    (`self.OnIncreseHealthEventDispatcher`)
    (else
      (`self.OnDecreseHealthEventDispatcher`)
      (`self.DeadCheck`))))

(event `UpdateCurrHealthInMax`
  (`self.SetCurrHealth` (`KismetMathLibrary.Clamp` (`self.CurrHealth`) 0 (`self.MaxHealth`))))

(event `AdjustHealthPercent`
  (params (Percent :type Integer))
  (`self.AdjustHealth` (* (/ Percent 100.0) (`self.MaxHealth`))))

(fn `DeadCheck`
  (bind _output_get (set `self.bDead?` (<= (`self.CurrHealth`) 0)))
  (if _output_get
    (`self.OnDeadEventDispatcher`)))

(fn `Get Health Info`
  (returns (CurrHealth :type Integer) (MaxHealth :type Integer))
  (return (`self.CurrHealth`) (`self.MaxHealth`)))

(fn `GetPercent`
  (returns (ReturnValue :type "Float (double-precision)"))
  (locals (ProgressBar :type "ProgressBar Object Reference"))
  (return (/ (`self.CurrHealth`) (`self.MaxHealth`))))

(fn `MultMaxHealth`
  (params (adjust :type "Float (double-precision)"))
  (locals (BeforeMaxHealth :type Integer :default 0))
  (bind _returnvalue (`KismetMathLibrary.FTrunc` (`/Game/Blueprints/BPFL_etc.Get Mult Adjusted (increase)` (`KismetMathLibrary.Conv_IntToDouble` (`self.StartMaxHealth`)) adjust)))
  (bind _returnvalue_2 (`KismetMathLibrary.Clamp` _returnvalue 1 _returnvalue))
  (bind _returnvalue_3 (- _returnvalue_2 (`local.BeforeMaxHealth`)))
  (set `local.BeforeMaxHealth` (`self.MaxHealth`))
  (set `self.MaxHealth` _returnvalue_2)
  (if (> _returnvalue_3 0)
    (`self.AdjustHealth` _returnvalue_3)))