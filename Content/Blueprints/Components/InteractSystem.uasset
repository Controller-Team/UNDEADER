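; Interaction component that tracks the closest interactable item near its owner and forwards interaction attempts to it.
; Each tick a sphere overlap gathers BP_InteractableBase actors within InteractRange, then retargets to the nearest or clears a target no longer found.
; Target changes notify the old and new items through unset and set callbacks, and TryInteract calls Interact on the current target.
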(event `Try Interact`
  (params (Interacter :type "/Game/Blueprints/PlayerCharacter/BP_PlayerCharacter Object Reference"))
  (bind _curr_interact_target_item (`self.Curr Interact Target Item`))
  (`/Engine/EditorBlueprintResources/StandardMacros.IsValid` _curr_interact_target_item
    (:`Is Valid`
      (`/Game/Blueprints/Interactables/BP_InteractableBase.Interact` _curr_interact_target_item Interacter))))

(event `self.ReceiveTick`
  (params (DeltaSeconds :type "Float (single-precision)"))
  (bind _asitem_base (`self.Get Closet Item`))
  (bind _asitem_base_2 (`self.Get Closet Item`))
  (set `self.ItemActorsInRange` (`self.GetItemArr`))
  (`/Engine/EditorBlueprintResources/StandardMacros.IsValid` (`self.Curr Interact Target Item`)
    (:`Is Valid`
      (if (`self.Check Item In Range`)
        (`/Engine/EditorBlueprintResources/StandardMacros.IsValid` _asitem_base
          (:`Is Valid`
            (if (!= _asitem_base (`self.Curr Interact Target Item`))
              (`self.Set Interact Target` _asitem_base))))
        (else
          (`self.Set Interact Target` null))))
    (:`Is Not Valid`
      (`/Engine/EditorBlueprintResources/StandardMacros.IsValid` _asitem_base_2
        (:`Is Valid`
          (`self.Set Interact Target` _asitem_base_2))))))

(fn `Check Item In Range`
  (returns (ReturnValue :type Boolean))
  (for _array_element (`self.ItemActorsInRange`)
    (if (== (`Actor.GetOwner` _array_element) (`Actor.GetOwner` (`self.Curr Interact Target Item`)))
      (return true)))
  (return false))

(fn `Get Closet Item`
  (returns (`AsItem Base` :type "/Game/Blueprints/Interactables/BP_InteractableBase Object Reference"))
  (locals (`Closest idx` :type Integer) (`closest range` :type "Float (double-precision)"))
  (bind _itemactorsinrange (`self.ItemActorsInRange`))
  (set `local.closest range` (`self.InteractRange`))
  (if (> (`KismetArrayLibrary.Array_Length` _itemactorsinrange) 0)
    (for (_array_element _array_index) _itemactorsinrange
      (cast `/Game/Blueprints/Interactables/BP_InteractableBase` _array_element)
      (bind _returnvalue (`KismetMathLibrary.Vector_Distance` (`Actor.K2_GetActorLocation` (`self.GetOwner`)) (`Actor.K2_GetActorLocation` _array_element)))
      (if (< _returnvalue (`local.closest range`))
        (set `local.closest range` _returnvalue)
        (set `local.Closest idx` _array_index)))
    (bind _asbp_interactable_base (cast `/Game/Blueprints/Interactables/BP_InteractableBase` (`|GetArrayItem` _itemactorsinrange (`local.Closest idx`))))
    (return _asbp_interactable_base)
    (else
      (return null))))

(fn `GetItemArr`
  (returns (OutActors :type "Array of Actor Object Reference"))
  (bind _outactors (`KismetSystemLibrary.SphereOverlapActors` (`Actor.K2_GetActorLocation` (`self.GetOwner`)) (`self.InteractRange`) (`self.Item Object Types`) "/Game/Blueprints/Interactables/BP_InteractableBase.BP_InteractableBase_C"))
  (return _outactors))

(fn `Set Interact Target`
  (params (item :type "/Game/Blueprints/Interactables/BP_InteractableBase Object Reference"))
  (bind _curr_interact_target_item (`self.Curr Interact Target Item`))
  (`|ExecutionSequence`
    (:`then_0`
      (`/Engine/EditorBlueprintResources/StandardMacros.IsValid` _curr_interact_target_item
        (:`Is Valid`
          (`/Game/Blueprints/Interactables/BP_InteractableBase.On Unset Interact Target` _curr_interact_target_item))))
    (:`then_1`
      (bind _output_get (set `self.Curr Interact Target Item` item))
      (`/Engine/EditorBlueprintResources/StandardMacros.IsValid` _output_get
        (:`Is Valid`
          (`/Game/Blueprints/Interactables/BP_InteractableBase.On Set Interact Target` _output_get))))))