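; Component that keeps the nearest BP_ItemBase within range of its owner as the interact target and forwards TryInteract to it.
; Each tick, a sphere overlap finds the closest item, and target changes notify the old and new items.
; The current target's range is checked by a multi line trace toward it, matching actor owners rather than the actors themselves.
; Debug shapes and target-change prints are left on.
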(event `Try Interact`
  (params (Interacter :type "/Game/Blueprints/PlayerCharacter/BP_PlayerCharacter Object Reference"))
  (bind _curr_interact_target_item (`self.Curr Interact Target Item`))
  (`/Engine/EditorBlueprintResources/StandardMacros.IsValid` _curr_interact_target_item
    (:`Is Valid`
      (`/Game/Blueprints/Items/BP_ItemBase.Interact` _curr_interact_target_item Interacter))))

(event `self.ReceiveTick`
  (params (DeltaSeconds :type "Float (single-precision)"))
  (bind _asitem_base (`self.Get Closet Item`))
  (bind _asitem_base_2 (`self.Get Closet Item`))
  (`/Engine/EditorBlueprintResources/StandardMacros.IsValid` (`self.Curr Interact Target Item`)
    (:`Is Valid`
      (if (`self.Check Item In Range`)
        (`/Engine/EditorBlueprintResources/StandardMacros.IsValid` _asitem_base
          (:`Is Valid`
            (if (!= _asitem_base (`self.Curr Interact Target Item`))
              (`self.Set Interact Target` _asitem_base))))
        (else
          (`self.Set Interact Target` null))))
    (:`Is Not Valid`
      (`/Engine/EditorBlueprintResources/StandardMacros.IsValid` _asitem_base_2
        (:`Is Valid`
          (`self.Set Interact Target` _asitem_base_2))))))

(fn `Check Item In Range`
  (returns (ReturnValue :type Boolean))
  (bind _returnvalue (`Actor.K2_GetActorLocation` (`self.GetOwner`)))
  (bind _outhits (`KismetSystemLibrary.LineTraceMultiForObjects` :`Start` _returnvalue :`End` (+ _returnvalue (* (`self.InteractRange`) (`KismetMathLibrary.Normal` (- (`Actor.K2_GetActorLocation` (`self.Curr Interact Target Item`)) _returnvalue))) (0.0 0.0 0.0)) :`ObjectTypes` (`self.Item Object Types`) :`DrawDebugType` "ForOneFrame"))
  (for _array_element _outhits
    (if (== (`Actor.GetOwner` (`.HitActor` (`GameplayStatics.BreakHitResult` _array_element))) (`Actor.GetOwner` (`self.Curr Interact Target Item`)))
      (return true)))
  (return false))

(fn `Get Closet Item`
  (returns (`AsItem Base` :type "/Game/Blueprints/Items/BP_ItemBase Object Reference"))
  (locals (`Closest idx` :type Integer) (`closest range` :type "Float (double-precision)"))
  (bind _interactrange (`self.InteractRange`))
  (bind _returnvalue (`Actor.K2_GetActorLocation` (`self.GetOwner`)))
  (set `local.closest range` (`self.InteractRange`))
  (bind (_outactors _returnvalue_2) (`KismetSystemLibrary.SphereOverlapActors` _returnvalue _interactrange (`self.Item Object Types`) "/Game/Blueprints/Items/BP_ItemBase.BP_ItemBase_C"))
  (`KismetSystemLibrary.DrawDebugSphere` _returnvalue _interactrange 12 (struct :`G` 0.033423 :`B` 1.0 :`A` 1.0))
  (if _returnvalue_2
    (for (_array_element _array_index) _outactors
      (cast `/Game/Blueprints/Items/BP_ItemBase` _array_element)
      (bind _returnvalue_3 (`KismetMathLibrary.Vector_Distance` (`Actor.K2_GetActorLocation` (`self.GetOwner`)) (`Actor.K2_GetActorLocation` _array_element)))
      (if (< _returnvalue_3 (`local.closest range`))
        (set `local.closest range` _returnvalue_3)
        (set `local.Closest idx` _array_index)))
    (bind _asbp_item_base (cast `/Game/Blueprints/Items/BP_ItemBase` (`|GetArrayItem` _outactors (`local.Closest idx`))))
    (return _asbp_item_base)
    (else
      (return null))))

(fn `Set Interact Target`
  (params (item :type "/Game/Blueprints/Items/BP_ItemBase Object Reference"))
  (bind _curr_interact_target_item (`self.Curr Interact Target Item`))
  (`|ExecutionSequence`
    (:`then_0`
      (`/Engine/EditorBlueprintResources/StandardMacros.IsValid` _curr_interact_target_item
        (:`Is Valid`
          (`/Game/Blueprints/Items/BP_ItemBase.On Unset Interact Target` _curr_interact_target_item)
          (`KismetSystemLibrary.PrintString` (`KismetStringLibrary.Concat_StrStr` "change interact target: " "none")))))
    (:`then_1`
      (bind _output_get (set `self.Curr Interact Target Item` item))
      (`/Engine/EditorBlueprintResources/StandardMacros.IsValid` _output_get
        (:`Is Valid`
          (`/Game/Blueprints/Items/BP_ItemBase.On Set Interact Target` _output_get)
          (bind _iteminfo_itemname (break `/Game/Blueprints/Items/ItemInfo` (`/Game/Blueprints/Items/BP_ItemBase.ItemInfo` _output_get)))
          (`KismetSystemLibrary.PrintString` (`KismetStringLibrary.Concat_StrStr` "change interact target: " _iteminfo_itemname)))))))