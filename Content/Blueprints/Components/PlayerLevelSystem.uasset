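; Player component that tracks level and experience, with an init event to set both values.
; Gained experience is added, then a level-up check loops to carry surplus over multiple levels against a requirement that grows linearly with level.
; Each level-up increments the level and calls OnLevelUp.
; After each gain, it pushes level and experience to the HUD bottom bar through BP_ThirdPersonGameMode.
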(event `InitLevelSystem`
  (params (CurrLevel :type Integer) (CurrExp :type Integer))
  (set `self.CurrLevel` CurrLevel)
  (set `self.CurrExp` CurrExp))

(event `self.ReceiveBeginPlay`
  (`KismetSystemLibrary.PrintString` (`KismetStringLibrary.Conv_IntToString` (`self.GetExpToNextLevel`)) true true (struct :`R` 0.883538 :`G` 1.0 :`B` 0.948436 :`A` 1.0)))

(event `GetExp`
  (params (amount :type Integer))
  (set `self.CurrExp` (+ amount (`self.CurrExp`)))
  (`self.CheckLevelUp`)
  (`self.Update Level and Exp UI`))

(event `CheckLevelUp`
  (if (>= (`self.CurrExp`) (`self.GetExpToNextLevel`)) :!label _label
    (set `self.CurrExp` (- (`self.CurrExp`) (`self.GetExpToNextLevel`)))
    (`self.LevelUp`)
    (goto _label)))

(event `LevelUp`
  (`/Engine/EditorBlueprintResources/StandardMacros.IncrementInt` (`self.CurrLevel`)
    (:`  `
      (`KismetSystemLibrary.PrintString` "Player LevelUp" true true (struct :`R` 1.0 :`B` 0.68754 :`A` 1.0))
      (`self.OnLevelUp`))))

(event `Update Level and Exp UI`
  (bind _bottombar (`/Game/Blueprints/WBP/WBP_HUD.BottomBar` (`/Game/Blueprints/BP_ThirdPersonGameMode.WBP HUD` (cast `/Game/Blueprints/BP_ThirdPersonGameMode` (`GameplayStatics.GetGameMode`) :!pure true))))
  (`/Game/Blueprints/WBP/HUD/WBP_BottomBar.SetLevelUI` _bottombar (`self.CurrLevel`))
  (`/Game/Blueprints/WBP/HUD/WBP_BottomBar.SetExpUI` _bottombar (`self.CurrExp`) (`self.GetExpToNextLevel`)))

(fn `GetCurrExp`
  (returns (CurrExp :type Integer))
  (return (`self.CurrExp`)))

(fn `GetCurrLvl`
  (returns (CurrLevel :type Integer))
  (return (`self.CurrLevel`)))

(fn `GetExpToNextLevel`
  (returns (ReturnValue :type Integer))
  (return (+ (* (`self.CurrLevel`) 50) 50)))