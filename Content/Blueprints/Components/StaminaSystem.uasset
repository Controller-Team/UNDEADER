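; Stamina component that holds an integer stamina pool, handles spending it and regenerates it over time.
; UseStamina returns false after a successful spend and true when stamina is insufficient.
; Each spend restarts a looping timer that restores one point per tick, at an interval derived from the default delay and multiplier.
; All changes are clamped between zero and max, then broadcast through the AdjustStamina event dispatcher.
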(event `InitStamina`
  (params (MaxStamina :type Integer))
  (bind _output_get (set `self.MaxStamina` MaxStamina))
  (set `self.CurrStamin` _output_get))

(event `WaitRestore`
  (params (Time :type "Float (single-precision)"))
  (`KismetSystemLibrary.K2_ClearAndInvalidateTimerHandle` (`self.RestoerTimer`))
  (bind _returnvalue (`KismetSystemLibrary.K2_SetTimerDelegate` (delegate `Restore`) Time true))
  (set `self.RestoerTimer` _returnvalue))

(event `Restore`
  (`self.AdujstStamina` 1))

(fn `AdujstStamina`
  (params (adjust :type Integer))
  (set `self.CurrStamin` (`KismetMathLibrary.Clamp` (+ adjust (`self.CurrStamin`)) 0 (`self.MaxStamina`)))
  (`self.AdjustStaminaED`))

(fn `Get CurrStamina`
  (returns (CurrStamin :type Integer))
  (return (`self.CurrStamin`)))

(fn `Use Stamina`
  (params (Usage :type Integer))
  (returns (`bFail?` :type Boolean))
  (if (>= (`self.CurrStamin`) Usage)
    (`self.AdujstStamina` (* Usage -1))
    (`self.WaitRestore` (`/Game/Blueprints/BPFL_etc.Get Mult Adjusted (decrease)` (`self.ResDelayDefault`) (`self.ResDelayMult`)))
    (return false)
    (else
      (return true))))