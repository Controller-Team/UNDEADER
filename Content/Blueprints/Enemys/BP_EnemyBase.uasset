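; Base enemy character that chases the player, makes melee zombie attacks and ragdolls on death.
; Tick moves it toward the player via AIMoveTo and starts an attack when the player overlaps its Box.
; Attacks wait until the AnimBP stops moving, then play a montage whose notify calls AttackHit to damage an overlapping player.
; HealthSystem dispatchers drive the health widget, a brief overlay-material hit flash and the death handling.
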(event `InitHealthSystem`
  ;[1 1 1] Init HealthSystem
  (`/Game/Blueprints/Components/HealthSystem.InitHealthSystem` (`self.HealthSystem`)))

(event `UpdateHealthUI`
  ;[1 1 1] Init HealthSystem
  (bind _aswbp_health_gage (cast `/Game/ThirdPerson/UI/WBP_HealthGage` (`WidgetComponent.GetWidget` (`self.HealthGage`))))
  (`ProgressBar.SetPercent` (`/Game/ThirdPerson/UI/WBP_HealthGage.ProgressBar_84` _aswbp_health_gage) (`/Game/Blueprints/Components/HealthSystem.GetPercent` (`self.HealthSystem`))))

(event `self.ReceiveBeginPlay`
  (`self.InitHealthSystem`))

(event `ToggleHealthUI`
  (params (toggle :type Boolean))
  (bind _returnvalue (`WidgetComponent.GetWidget` (`self.HealthGage`)))
  (if toggle
    (`Widget.SetVisibility` _returnvalue "Visible")
    (else
      (`Widget.SetVisibility` _returnvalue "Hidden"))))

(event `SetMaxMoveSpeed`
  (params (`Max Walk Speed` :type "Float (single-precision)"))
  (set `CharacterMovementComponent.MaxWalkSpeed` `Max Walk Speed` (`self.CharacterMovement`)))

(event `self.HealthSystem.OnDecreseHealthEventDispatcher`
  ;[1 1 1] Init HealthSystem
  (`self.UpdateHealthUI`)
  (`self.HitEffect`))

(event `self.ReceiveTick`
  (params (DeltaSeconds :type "Float (single-precision)"))
  (`|ExecutionSequence`
    (:`then_0`
      (`self.Target In Range` "/Game/Blueprints/PlayerCharacter/BP_PlayerCharacter.BP_PlayerCharacter_C"
        (:`true`
          (`self.AttackCheck`))))
    (:`then_1`
      (if (not (`/Game/Blueprints/Components/HealthSystem.bDead?` (`self.HealthSystem`)))
        (if (not (`self.bAttacking?`))
          (`self.FollowPlayer`)
          (else
            (`|AIMoveTo` self (`self.K2_GetActorLocation`) null)))))))

(event `FollowPlayer`
  (`|AIMoveTo` self (`self.K2_GetActorLocation` (`GameplayStatics.GetPlayerCharacter` 0)) null))

(event `self.HealthSystem.OnDeadEventDispatcher`
  (bind _mesh (`self.Mesh`))
  ;[1 1 1] Init HealthSystem
  (`PrimitiveComponent.SetCollisionEnabled` _mesh "PhysicsOnly")
  (`PrimitiveComponent.SetSimulatePhysics` _mesh true)
  (`self.ToggleHealthUI` false)
  (`PrimitiveComponent.SetCollisionEnabled` (`self.CapsuleComponent`) "NoCollision")
  (`SkeletalMeshComponent.Stop` (`self.Mesh`)))

(event `self.HealthSystem.OnInitEventDispatcher`
  ;[1 1 1] Init HealthSystem
  (`self.UpdateHealthUI`))

(event `AttackCheck`
  (bind _alphablendargs (make `AlphaBlendArgs` null 0.2 "CubicInOut"))
  (if (not (`self.bAttacking?`))
    (set `self.bAttacking?` true)
    (bind _asabp_enemy (cast `/Game/Blueprints/Enemys/ABP_Enemy` (`SkeletalMeshComponent.GetAnimInstance` (`self.Mesh`))))
    (`KismetSystemLibrary.DelayUntilNextTick` :!label _label)
    (if (not (`/Game/Blueprints/Enemys/ABP_Enemy.ShouldMove` _asabp_enemy))
      (bind _returnvalue (`AnimInstance.Montage_PlayWithBlendIn` _asabp_enemy "/Game/BSP_ZombieAnims/Animations/Standing/Attack/AM_zombieAttack.AM_zombieAttack" _alphablendargs (`self.In Play Rate`) "Duration" 0.0 true))
      (`KismetSystemLibrary.Delay` _returnvalue)
      (`AnimInstance.Montage_StopWithBlendOut` _asabp_enemy _alphablendargs "/Game/BSP_ZombieAnims/Animations/Standing/Attack/AM_zombieAttack.AM_zombieAttack")
      (set `self.bAttacking?` false)
      (else
        (goto _label)))))

(event `AttackHit`
  (bind _returnvalue (`GameplayStatics.GetPlayerCharacter` 0))
  (if (`PrimitiveComponent.IsOverlappingActor` (`self.Box`) _returnvalue)
    (bind _asbp_player_character (cast `/Game/Blueprints/PlayerCharacter/BP_PlayerCharacter` _returnvalue))
    (`/Game/Blueprints/Components/HealthSystem.AdjustHealth` (`/Game/Blueprints/PlayerCharacter/BP_PlayerCharacter.HealthSystem` _asbp_player_character) -10)))

(event `HitEffect`
  (bind _mesh (`self.Mesh`))
  (`MeshComponent.SetOverlayMaterial` _mesh "/Game/Overlay/M_Overlay.M_Overlay")
  (`KismetSystemLibrary.Delay` 0.15)
  (`MeshComponent.SetOverlayMaterial` _mesh null))

(fn `GetBounds`
  (returns (Origin :type "Vector Structure") (BoxExtent :type "Vector Structure"))
  (bind (_origin _boxextent) (`self.GetActorBounds` false))
  (return _origin _boxextent))

(fn `UserConstructionScript`)