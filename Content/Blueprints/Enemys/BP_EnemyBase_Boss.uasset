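; Boss enemy base Blueprint that extends a parent enemy with a screen HP bar and clears the game when killed.
; From BeginPlay, a one-second Delay loop drains the player's HealthSystem by ContinuousDamage, regardless of distance, while that component is valid.
; InitHealthUI adds the boss bar widget to the viewport, and UpdateHealthUI feeds it current and starting max health.
; OnKilled calls GameClear on the GameMode's level manager.
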(event `self.ReceiveBeginPlay`
  (`parent.ReceiveBeginPlay`)
  (set `self.Overlay Mesh Target` (`self.Synty Mesh`))
  (`self.DoContinuousDamage`))

(event `self.ReceiveTick`
  (params (DeltaSeconds :type "Float (single-precision)"))
  (`parent.ReceiveTick` DeltaSeconds))

(event `DoContinuousDamage`
  (bind _healthsystem (`/Game/Blueprints/PlayerCharacter/BP_PlayerCharacter.HealthSystem` (`/Game/Blueprints/BPFL_etc.GetBP_PlayerCharacter` self)))
  (`/Engine/EditorBlueprintResources/StandardMacros.IsValid` _healthsystem :!label _label
    (:`Is Valid`
      (`/Game/Blueprints/Components/HealthSystem.AdjustHealth` _healthsystem (* (`self.continuousDamage`) -1) false false (struct :`R` 1.0 :`A` 1.0))
      (`KismetSystemLibrary.Delay` 1.0)
      (goto _label))))

(fn `InitHealthUI`
  (bind _returnvalue (`|CreateWidget` "/Game/Blueprints/WBP/HUD/WBP_BossHPBar.WBP_BossHPBar_C"))
  (bind _output_get (set `self.bossHpBar` _returnvalue))
  (`UserWidget.AddToViewport` _output_get 0)
  (`self.UpdateHealthUI`)
  (`parent.InitHealthUI`))

(fn `OnKilled`
  (params (bGetReward :type Boolean))
  (`parent.OnKilled` bGetReward)
  (`/Game/Blueprints/Level/BP_LevelManager.GameClear` (`/Game/Blueprints/BP_ThirdPersonGameMode.BP_LevelManager` (cast `/Game/Blueprints/BP_ThirdPersonGameMode` (`GameplayStatics.GetGameMode`) :!pure true))))

(fn `UpdateHealthUI`
  (bind _bosshpbar (`self.bossHpBar`))
  (bind _healthsystem (`self.HealthSystem`))
  (`/Engine/EditorBlueprintResources/StandardMacros.IsValid` _bosshpbar
    (:`Is Valid`
      (`/Game/Blueprints/WBP/HUD/WBP_BossHPBar.SetBossHPUI` _bosshpbar (`/Game/Blueprints/Components/HealthSystem.CurrHealth` _healthsystem) (`/Game/Blueprints/Components/HealthSystem.StartMaxHealth` _healthsystem)))))

(fn `UserConstructionScript`
  (`parent.UserConstructionScript`))