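; Game instance that builds the run's stage map on Init, giving two area-type choices per stage, and tracks the current area count and type.
; Choices draw from three random difficulty types, rerolling excluded ones.
; Accumulating pity odds may replace one random choice with a shop or, failing that, a rest area, resetting after each hit.
; Both choices on the first and last stages are then forced to fixed types.
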(event `self.ReceiveInit`
  (`self.Init Areas`)
  (`KismetSystemLibrary.PrintString` "Hello"))

(fn `Get Cur Level Type`
  (returns (CurrAreaType :type "/Game/Blueprints/Level/AreaType Enum"))
  (return (`self.CurrAreaType`)))

(fn `Get Curr Level Count`
  (returns (CurrLevel :type Integer))
  (return (`self.CurrAreaCount`)))

(fn `GetNextAreaType`
  (returns (choice1 :type "/Game/Blueprints/Level/AreaType Enum") (choice2 :type "/Game/Blueprints/Level/AreaType Enum"))
  (locals (area1type :type "/Game/Blueprints/Level/AreaType Enum" :default "NewEnumerator0") (area2type :type "/Game/Blueprints/Level/AreaType Enum" :default "NewEnumerator0") (exceptTypeArr :type "Array of /Game/Blueprints/Level/AreaType Enum"))
  (bind _output_get (set `local.area1type` (`self.GetRandomAreaDifficult` (`local.exceptTypeArr`))))
  (set `local.area2type` (`self.GetRandomAreaDifficult` _output_get))
  (return (`local.area1type`) (`local.area2type`)))

(fn `GetRandomAreaDifficult`
  (params (exceptType :type "Array of /Game/Blueprints/Level/AreaType Enum"))
  (returns (`_ran type` :type "/Game/Blueprints/Level/AreaType Enum"))
  (locals (`execpt type` :type "Array of /Game/Blueprints/Level/AreaType Enum") (`ran type` :type "/Game/Blueprints/Level/AreaType Enum" :default "NewEnumerator0"))
  (set `local.execpt type` exceptType)
  (switch `int` (`KismetMathLibrary.RandomInteger` 3) :!label _label ; 무작위 난이도 구역 타입 구하기
    (:`0`
      (set `local.ran type` "NewEnumerator0"))
    (:`1`
      (set `local.ran type` "NewEnumerator1"))
    (:`2`
      (set `local.ran type` "NewEnumerator2")))
  (if (`KismetArrayLibrary.Array_Contains` (`local.execpt type`) (`local.ran type`))
    (goto _label)
    (else
      (return (`local.ran type`)))))

(fn `Init Areas`
  (locals (areaIdx :type Integer) (LastStageIdx :type Integer :default 14))
  (bind (_choice1 _choice2) (`self.GetNextAreaType`))
  (`|ExecutionSequence`
    (:`then_0`
      (for _index (range (+ (`local.LastStageIdx`) 1))
        (bind _output_get (set `local.areaIdx` _index))
        (`KismetArrayLibrary.Array_Set` (`self.AreaChoice1List`) _output_get _choice1 true)
        (`KismetArrayLibrary.Array_Set` (`self.AreaChoice2List`) _output_get _choice2 true)
        (if (> (`self.ShopAdventPercent`) (`KismetMathLibrary.RandomInteger` 100))
          (`self.OverrideSingleAreaType` (`local.areaIdx`) "NewEnumerator3")
          (set `self.ShopAdventPercent` 0)
          (else
            (set `self.ShopAdventPercent` (+ (`self.ShopAdventPercent`) 20))
            (if (> (`self.RestAdventPercent`) (`KismetMathLibrary.RandomInteger` 100))
              (`self.OverrideSingleAreaType` (`local.areaIdx`) "NewEnumerator4")
              (set `self.RestAdventPercent` 0)
              (else
                (set `self.RestAdventPercent` (+ (`self.RestAdventPercent`) 20))))))))
    (:`then_2`
      (`self.OverrideAllAreaType` 0)
      (`self.OverrideAllAreaType` (`local.LastStageIdx`) "NewEnumerator5"))))

(fn `OverrideAllAreaType`
  (params (areaCount :type Integer) (areaType :type "/Game/Blueprints/Level/AreaType Enum" :default "NewEnumerator0"))
  (`KismetArrayLibrary.Array_Set` (`self.AreaChoice1List`) areaCount areaType true)
  (`KismetArrayLibrary.Array_Set` (`self.AreaChoice2List`) areaCount areaType true))

(fn `OverrideSingleAreaType`
  (params (areaCount :type Integer) (areaType :type "/Game/Blueprints/Level/AreaType Enum" :default "NewEnumerator0"))
  (if (`KismetMathLibrary.RandomBool`)
    (`KismetArrayLibrary.Array_Set` (`self.AreaChoice1List`) areaCount areaType true)
    (else
      (`KismetArrayLibrary.Array_Set` (`self.AreaChoice2List`) areaCount areaType true))))

(fn `Update Area Info`
  (params (NextAreaCount :type "Integer (by ref)") (NextAreaTypr :type "/Game/Blueprints/Level/AreaType Enum" :default "NewEnumerator0"))
  (returns (CurrLevel :type Integer))
  (bind _output_get (set `self.CurrAreaCount` NextAreaCount))
  (set `self.CurrAreaType` NextAreaTypr)
  (return _output_get))