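; Accessory pickup item that starts hidden, becomes visible on ChestOpen, and wraps a BP_AccessoryBase child actor holding the accessory's data.
; InitAccItem passes accessory data into that child actor.
; On TakeItem, a new BP_AccessoryBase is spawned on the interactor's AccList with copied attributes and upgrade level, registered with its AccessorySystem, then attributes update and the pickup is disabled.
; BeginPlay also prints the damage multiplier for debugging.
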(event `ToggleItemVisible`
  (params (bVisible :type Boolean))
  (`SceneComponent.SetHiddenInGame` (`self.BP_AccessoryBase`) (not bVisible) true))

(event `self.ReceiveBeginPlay`
  (`self.SetItemInfoDefault`)
  (`self.ToggleItemVisible` false)
  (bind _asbp_accessory_base (cast `/Game/Blueprints/Accessorys/BP_AccessoryBase` (`ChildActorComponent.ChildActor` (`self.BP_AccessoryBase`))))
  (`KismetSystemLibrary.PrintString` (`KismetStringLibrary.Conv_DoubleToString` (`.DamageMult_6_0675F0D94A596EA056FE63A0E0C7DC37` (break `/Game/Blueprints/Accessorys/AdditionalAttribute` (`/Game/Blueprints/Accessorys/BP_AccessoryBase.DefaultAttribute` _asbp_accessory_base)))) true true (struct :`G` 1.0 :`B` 0.040663 :`A` 1.0)))

(event `SetItemInfoDefault`)

(event `InitAccItem`
  (params (`acc data` :type "/Game/Blueprints/DataStructure/AccData Structure"))
  (bind _asbp_accessory_base (cast `/Game/Blueprints/Accessorys/BP_AccessoryBase` (`ChildActorComponent.ChildActor` (`self.BP_AccessoryBase`))))
  (`/Game/Blueprints/Accessorys/BP_AccessoryBase.InitAcc` _asbp_accessory_base `acc data`))

(fn `AttachAcc`
  (params (Parent :type "SceneComponent Object Reference"))
  (returns (`Attached Acc` :type "/Game/Blueprints/Accessorys/BP_AccessoryBase Object Reference"))
  (bind (_defaultattribute _addattributeperlevel _upgradelevel) (`/Game/Blueprints/Accessorys/BP_AccessoryBase.GetAccInfo` (cast `/Game/Blueprints/Accessorys/BP_AccessoryBase` (`ChildActorComponent.ChildActor` (`self.BP_AccessoryBase`)) :!pure true)))
  (bind _returnvalue (`|SpawnActorFromClass` "/Game/Blueprints/Accessorys/BP_AccessoryBase.BP_AccessoryBase_C" (`KismetMathLibrary.MakeTransform` (0.0 0.0 0.0)) "AlwaysSpawn" "MultiplyWithRoot" (`ActorComponent.GetOwner` Parent) null))
  (`self.K2_AttachToComponent` _returnvalue Parent "None" "KeepRelative" "KeepRelative" "KeepRelative" true)
  (`/Game/Blueprints/Accessorys/BP_AccessoryBase.InitAccInfo` _returnvalue _defaultattribute _addattributeperlevel _upgradelevel)
  (return _returnvalue))

(fn `ChestOpen`
  (`parent.ChestOpen`)
  (`self.ToggleItemVisible` true))

(fn `TakeItem`
  (params (m_interactor :type "/Game/Blueprints/PlayerCharacter/BP_PlayerCharacter Object Reference"))
  (bind _attached_acc (`self.AttachAcc` (`/Game/Blueprints/PlayerCharacter/BP_PlayerCharacter.AccList` m_interactor)))
  (`/Game/Blueprints/Components/AccessorySystem.TakeAcc` (`/Game/Blueprints/PlayerCharacter/BP_PlayerCharacter.AccessorySystem` m_interactor) _attached_acc)
  (`/Game/Blueprints/PlayerCharacter/BP_PlayerCharacter.UpdateAttribute` m_interactor)
  (`self.DisableItem` (`self.BP_AccessoryBase`)))

(fn `UserConstructionScript`
  (`parent.UserConstructionScript`))