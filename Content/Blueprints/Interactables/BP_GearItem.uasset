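; BP_GearItem is an interactable pickup that grants an amount of gear to the player's resources.
; Init stores the amount, and TakeItem passes it to the resource manager's TryAdjustGear, then disables the item through its MoneyMesh.
; SelectChest extends the parent's version by prop type, showing MoneyMesh for Stone and hiding it for the three chest tiers.
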(event `Init`
  (params (Amount :type Integer))
  (set `self.Amount` Amount))

(fn `SelectChest`
  (params (propType :type "/Game/Blueprints/Interactables/ItemPropType Enum" :default "NewEnumerator0"))
  (bind _moneymesh (`self.moneyMesh`))
  (`parent.SelectChest` propType)
  (switch `/Game/Blueprints/Interactables/ItemPropType` propType
    (:`NewEnumerator1`
      (`SceneComponent.SetVisibility` _moneymesh true true))
    (:`NewEnumerator2`
      (`SceneComponent.SetVisibility` _moneymesh false false :!label _label))
    (:`NewEnumerator3`
      (goto _label))
    (:`NewEnumerator4`
      (goto _label))))

(fn `TakeItem`
  (params (m_interactor :type "/Game/Blueprints/PlayerCharacter/BP_PlayerCharacter Object Reference"))
  (`/Game/Blueprints/PlayerRes/BP_PlayerResManager.Try Adjust Gear` (`/Game/Blueprints/BPFL_etc.GetBP_ResManager` self) (`self.Amount`))
  (`self.DisableItem` (`self.moneyMesh`)))

(fn `UserConstructionScript`
  (`parent.UserConstructionScript`))