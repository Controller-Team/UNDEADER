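; BP_HealInteractable is an interactable that heals whoever interacts with it.
; Its Interact override calls the parent implementation, then passes HealAmount to AdjustHealth on the interacter's HealthSystem and returns the parent's result.
; The health change applies regardless of that result, and the event graph and construction script add no logic of their own.
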(fn `Interact`
  (params (interacter :type "/Game/Blueprints/PlayerCharacter/BP_PlayerCharacter Object Reference"))
  (returns (`bSuccess?` :type Boolean))
  (bind _bsuccess_ (`parent.Interact` interacter))
  (`/Game/Blueprints/Components/HealthSystem.AdjustHealth` (`/Game/Blueprints/PlayerCharacter/BP_PlayerCharacter.HealthSystem` interacter) (`self.HealAmount`))
  (return _bsuccess_))

(fn `UserConstructionScript`
  (`parent.UserConstructionScript`))