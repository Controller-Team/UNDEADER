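; BP_NPC is an interactable NPC that offers a random weapon or accessory reward and can be upgraded with gear.
; It spawns the reward through the game mode's reward manager at a configurable spawn point shortly after BeginPlay.
; Interacting spends gear at a cost that rises with NPC level.
; A successful upgrade raises the level and replaces any remaining item with a newly rolled one at the matching upgrade level.
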(event `self.ReceiveBeginPlay`
  (`KismetSystemLibrary.DelayUntilNextTick`)
  (`self.ProvideItem`))

(event `TryUpgadeNPC`
  (bind _spawned_item (`self.Spawned Item`))
  (bind _bsuccces_ (`/Game/Blueprints/PlayerRes/BP_PlayerResManager.Try Adjust Gear` (`/Game/Blueprints/BPFL_etc.GetBP_ResManager` self) (* (+ (`self.NpcUpgradeLevel`) 1) 2 -1)))
  (if _bsuccces_
    (bind _result (`/Engine/EditorBlueprintResources/StandardMacros.IncrementInt` (`self.NpcUpgradeLevel`))
      (:`  `
        (`/Engine/EditorBlueprintResources/StandardMacros.IsValid` _spawned_item ; 아이템이 존재하는 경우, 강화된 아이템으로 갱신
          (:`Is Valid`
            (`self.K2_DestroyActor` _spawned_item)
            (`self.ProvideItem`)))))))

(fn `Interact`
  (params (interacter :type "/Game/Blueprints/PlayerCharacter/BP_PlayerCharacter Object Reference"))
  (returns (`bSuccess?` :type Boolean))
  (bind _bsuccess_ (`parent.Interact` interacter))
  (`self.TryUpgadeNPC`)
  (return _bsuccess_))

(fn `ProvideItem`
  (locals (weaponPer :type Integer :default 0) (AccPer :type Integer :default 0))
  (bind _bp_rewardmanager (`/Game/Blueprints/BP_ThirdPersonGameMode.BP_RewardManager` (cast `/Game/Blueprints/BP_ThirdPersonGameMode` (`GameplayStatics.GetGameMode`) :!pure true)))
  (bind (_rewardtype _playerresamont _itemrarirty) (`/Game/Blueprints/Level/BP_RewardManager.Get Random Reward` _bp_rewardmanager (`local.weaponPer`) (`local.AccPer`) 0 0 34 33 33 0 0 0))
  (`|ExecutionSequence`
    (:`then_0`
      (switch `/Game/Blueprints/DataStructure/ItemType` (`self.provideItemType`)
        (:`NewEnumerator1`
          (set `local.AccPer` 100))
        (:`NewEnumerator2`
          (set `local.weaponPer` 100))))
    (:`then_1`
      (bind _spawn_item (`/Game/Blueprints/Level/BP_RewardManager.Spawn Reward` _bp_rewardmanager _rewardtype _playerresamont _itemrarirty (`SceneComponent.K2_GetComponentToWorld` (`self.SpawnPoint`))))
      (set `self.Spawned Item` _spawn_item)
      (`/Game/Blueprints/Interactables/Bp_ItemBase.TrySetUpgradeLevel` _spawn_item (- (`self.NpcUpgradeLevel`) 1))
      (`/Game/Blueprints/Interactables/Bp_ItemBase.SelectChest` _spawn_item "NewEnumerator1"))))

(fn `UserConstructionScript`
  (`parent.UserConstructionScript`)
  (`SkeletalMeshComponent.SetSkeletalMeshAsset` (`self.SyntySkeletalMesh`) (`self.Mesh`))
  (`SceneComponent.K2_SetRelativeLocation` (`self.SpawnPoint`) (`self.SpawnPointLocation`) false false))