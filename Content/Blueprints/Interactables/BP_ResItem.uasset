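; BP_ResItem is an interactable resource pickup that holds an amount of either Money or Gear.
; Taking it adds the amount through the resource manager, then destroys the actor.
; It extends parent chest logic by hiding its mesh in chest props until opened, while the Stone prop shows it immediately.
; As a shop item, it derives its price from the amount, with a large multiplier for Gear.
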(event `self.ReceiveBeginPlay`
  (`parent.ReceiveBeginPlay`))

(event `Init`
  (params (Amount :type Integer) (`item type` :type "/Game/Blueprints/DataStructure/ItemType Enum" :default "NewEnumerator3"))
  (bind _resmesh (`self.resMesh`))
  (set `self.Amount` Amount)
  (bind _output_get (set `self.Item Type` `item type`))
  (switch `/Game/Blueprints/DataStructure/ItemType` _output_get
    (:`NewEnumerator0`
      (`SkeletalMeshComponent.SetSkeletalMeshAsset` _resmesh "/Engine/EngineMeshes/SkeletalCube.SkeletalCube"))
    (:`NewEnumerator4`
      (`SkeletalMeshComponent.SetSkeletalMeshAsset` _resmesh "/Engine/EngineMeshes/SkeletalCube.SkeletalCube"))))

(fn `ChestOpen`
  (`parent.ChestOpen`)
  (`SceneComponent.SetVisibility` (`self.resMesh`) true true))

(fn `InitShopItem`
  (`parent.InitShopItem`)
  (switch `/Game/Blueprints/DataStructure/ItemType` (`self.Item Type`)
    (:`NewEnumerator0`
      (set `self.Price` (`self.Amount`)))
    (:`NewEnumerator4`
      (set `self.Price` (* (`self.Amount`) 10000)))))

(fn `SelectChest`
  (params (propType :type "/Game/Blueprints/Interactables/ItemPropType Enum" :default "NewEnumerator0"))
  (bind _resmesh (`self.resMesh`))
  (`parent.SelectChest` propType)
  (switch `/Game/Blueprints/Interactables/ItemPropType` propType
    (:`NewEnumerator1`
      (`SceneComponent.SetVisibility` _resmesh true true))
    (:`NewEnumerator2`
      (`SceneComponent.SetVisibility` _resmesh false false :!label _label))
    (:`NewEnumerator3`
      (goto _label))
    (:`NewEnumerator4`
      (goto _label))))

(fn `TakeItem`
  (params (m_interactor :type "/Game/Blueprints/PlayerCharacter/BP_PlayerCharacter Object Reference"))
  (bind _bp_playerresmanager (`/Game/Blueprints/BPFL_etc.GetBP_ResManager` self))
  (switch `/Game/Blueprints/DataStructure/ItemType` (`self.Item Type`)
    (:`NewEnumerator0`
      (`/Game/Blueprints/PlayerRes/BP_PlayerResManager.Try Adjust Money` _bp_playerresmanager (`self.Amount`)))
    (:`NewEnumerator4`
      (`/Game/Blueprints/PlayerRes/BP_PlayerResManager.Try Adjust Gear` _bp_playerresmanager (`self.Amount`))))
  (`self.K2_DestroyActor`))

(fn `UserConstructionScript`
  (`parent.UserConstructionScript`))