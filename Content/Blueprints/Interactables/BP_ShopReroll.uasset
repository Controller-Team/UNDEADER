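; BP_ShopReroll is an interactable that triggers a shop reroll and displays its price.
; One tick after BeginPlay, it caches the shop manager from BP_ThirdPersonGameMode and writes the manager's reroll price to its WBP_PriceTag widget.
; Interact runs the parent logic, asks the manager to attempt the reroll, then refreshes the displayed price.
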(event `self.ReceiveBeginPlay`
  (`KismetSystemLibrary.DelayUntilNextTick`)
  (set `self.BP Shop Manager` (`/Game/Blueprints/BP_ThirdPersonGameMode.BP_ShopManager` (cast `/Game/Blueprints/BP_ThirdPersonGameMode` (`GameplayStatics.GetGameMode`) :!pure true)))
  (`self.UpdatePriceUI`))

(event `UpdatePriceUI`
  (`/Game/Blueprints/WBP/HUD/WBP_PriceTag.SetPriceText` (cast `/Game/Blueprints/WBP/HUD/WBP_PriceTag` (`WidgetComponent.GetWidget` (`self.MoneyWidget`)) :!pure true) (`/Game/Blueprints/Level/BP_ShopManager.RerollPrice` (`self.BP Shop Manager`))))

(fn `Interact`
  (params (interacter :type "/Game/Blueprints/PlayerCharacter/BP_PlayerCharacter Object Reference"))
  (returns (`bSuccess?` :type Boolean))
  (bind _bsuccess_ (`parent.Interact` interacter))
  (`/Game/Blueprints/Level/BP_ShopManager.TryReroll` (`self.BP Shop Manager`))
  (`self.UpdatePriceUI`)
  (return _bsuccess_))

(fn `UserConstructionScript`
  (`parent.UserConstructionScript`))