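; BP_WeaponItem is an interactable weapon pickup that wraps a BP_MasterWeapon in a child actor component.
; On BeginPlay it takes its ammo and upgrade level from that weapon, defaulting to a full clip.
; SetWeaponInfo can override both values and prints the level to screen.
; Interact passes the child weapon, ammo and level to the interacter's ChangeSlotWeapon, then destroys the item.
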(event `self.ReceiveBeginPlay`
  (`self.SetWeaponInfoDefault`))

(event `self.Interact`
  (params (Interacter :type "/Game/Blueprints/PlayerCharacter/BP_PlayerCharacter Object Reference"))
  (bind _asbp_master_weapon (cast `/Game/Blueprints/Weapons/BP_MasterWeapon` (`ChildActorComponent.ChildActor` (`self.WeaponChild`))))
  (`/Game/Blueprints/PlayerCharacter/BP_PlayerCharacter.ChangeSlotWeapon` Interacter _asbp_master_weapon (`self.Left Ammo`) (`self.Upgrade Level`))
  (`self.K2_DestroyActor`))

(event `SetWeaponInfoDefault`
  (bind _asbp_master_weapon (cast `/Game/Blueprints/Weapons/BP_MasterWeapon` (`ChildActorComponent.ChildActor` (`self.WeaponChild`))))
  (set `self.Left Ammo` (`/Game/Blueprints/Weapons/BP_MasterWeapon.GetFullClipAmmo` _asbp_master_weapon)) ; 탄창이 가득 찬 상태 설정
  (set `self.Upgrade Level` (`/Game/Blueprints/Weapons/BP_MasterWeapon.GetCurrLevel` _asbp_master_weapon)))

(event `SetWeaponInfo`
  (params (LeftAmmo :type Integer) (`Upgrade Level` :type Integer))
  (set `self.Left Ammo` LeftAmmo)
  (bind _output_get (set `self.Upgrade Level` `Upgrade Level`))
  (`KismetSystemLibrary.PrintString` (`KismetStringLibrary.Conv_IntToString` _output_get) true true (struct :`R` 1.0 :`B` 0.734962 :`A` 1.0)))

(fn `UserConstructionScript`
  (`parent.UserConstructionScript`))