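; Base interactable for item pickups housed in a stone or one of three chest tiers.
; The first successful interaction plays the chest opening animations and clears prop overlay outlines; later ones call TakeItem, an empty hook here.
; Stone props count as already open, and retargeting an open prop clears its outlines again.
; SelectChest sets every prop mesh invisible, including the selected type, while DisableItem blocks interaction and hides a given component.
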(event `DisableItem`
  (params (hideComp :type "SceneComponent Object Reference"))
  (set `self.bCanInteract?` false)
  (`SceneComponent.SetHiddenInGame` hideComp true true))

(event `Chest Open Anim`
  (`SkeletalMeshComponent.PlayAnimation` (`self.Chest_Low`) "/Game/Maps/CoreObjects/Interact/SM_Prop_Chest_01_Skeleton_Sequence.SM_Prop_Chest_01_Skeleton_Sequence" false)
  (`SkeletalMeshComponent.PlayAnimation` (`self.Chest_Medium`) "/Game/Maps/CoreObjects/Interact/SM_Prop_Chest_02_Skeleton_Sequence.SM_Prop_Chest_02_Skeleton_Sequence" false)
  (`SkeletalMeshComponent.PlayAnimation` (`self.Chest_High`) "/Game/Maps/CoreObjects/Interact/SM_Prop_Chest_03_Skeleton_Sequence.SM_Prop_Chest_03_Skeleton_Sequence" false)
  (set `self.bChestOpen?` true))

(event `SelectChest`
  (params (propType :type "/Game/Blueprints/Interactables/ItemPropType Enum" :default "NewEnumerator0"))
  (`SceneComponent.SetVisibility` (`self.Stone`) false false)
  (`SceneComponent.SetVisibility` (`self.Chest_Low`) false false)
  (`SceneComponent.SetVisibility` (`self.Chest_Medium`) false false)
  (`SceneComponent.SetVisibility` (`self.Chest_High`) false false)
  (switch `/Game/Blueprints/Interactables/ItemPropType` propType
    (:`NewEnumerator1`
      (`SceneComponent.SetVisibility` (`self.Stone`) false false)
      (set `self.bChestOpen?` true))
    (:`NewEnumerator2`
      (`SceneComponent.SetVisibility` (`self.Chest_Low`) false false))
    (:`NewEnumerator3`
      (`SceneComponent.SetVisibility` (`self.Chest_Medium`) false false))
    (:`NewEnumerator4`
      (`SceneComponent.SetVisibility` (`self.Chest_High`) false false))))

(event `ExceptChestOutline`
  (for _array_element (`|MakeArray` (`self.Stone`) (`self.Chest_Low`) (`self.Chest_Medium`) (`self.Chest_High`))
    (`MeshComponent.SetOverlayMaterial` _array_element null)))

(fn `ChestOpen`
  (`self.Chest Open Anim`)
  (`self.ExceptChestOutline`))

(fn `Interact`
  (params (interacter :type "/Game/Blueprints/PlayerCharacter/BP_PlayerCharacter Object Reference"))
  (returns (`bSuccess?` :type Boolean))
  (locals (m_interactor :type "/Game/Blueprints/PlayerCharacter/BP_PlayerCharacter Object Reference"))
  (bind _bsuccess_ (`parent.Interact` interacter))
  (if _bsuccess_
    (if (`self.bChestOpen?`)
      (`self.TakeItem` interacter)
      (else
        (`self.ChestOpen`)))
    (return true)
    (else
      (return false))))

(fn `On Set Interact Target`
  (`parent.On Set Interact Target`)
  (if (`self.bChestOpen?`)
    (`self.ExceptChestOutline`)))

(fn `TakeItem`
  (params (m_interactor :type "/Game/Blueprints/PlayerCharacter/BP_PlayerCharacter Object Reference")))

(fn `UserConstructionScript`
  (`parent.UserConstructionScript`))