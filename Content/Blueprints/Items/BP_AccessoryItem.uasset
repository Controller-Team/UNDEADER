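; Pickup item that grants an accessory to whoever interacts with it.
; It holds the accessory as a BP_AccessoryBase child actor and reads that actor's Info.
; Interact passes the Info to the interacter's AccessorySystem, fires its OnGetItemEvent and destroys the pickup.
; BeginPlay calls the empty SetItemInfoDefault hook for default item state, then debug-prints the accessory's damage multiplier.
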(event `self.ReceiveBeginPlay`
  (`self.SetItemInfoDefault`)
  (bind _asbp_accessory_base (cast `/Game/Blueprints/Accessorys/BP_AccessoryBase` (`ChildActorComponent.ChildActor` (`self.BP_AccessoryBase`))))
  (`KismetSystemLibrary.PrintString` (`KismetStringLibrary.Conv_DoubleToString` (`.DamageMult_6_0675F0D94A596EA056FE63A0E0C7DC37` (break `/Game/Blueprints/Accessorys/AccessoryInfo` (`/Game/Blueprints/Accessorys/BP_AccessoryBase.Info` _asbp_accessory_base)))) true true (struct :`G` 1.0 :`B` 0.040663 :`A` 1.0)))

(event `self.Interact`
  (params (Interacter :type "/Game/Blueprints/PlayerCharacter/BP_PlayerCharacter Object Reference"))
  (bind _asbp_accessory_base (cast `/Game/Blueprints/Accessorys/BP_AccessoryBase` (`ChildActorComponent.ChildActor` (`self.BP_AccessoryBase`))))
  (`/Game/Blueprints/Components/AccessorySystem.AddAccessory` (`/Game/Blueprints/PlayerCharacter/BP_PlayerCharacter.AccessorySystem` Interacter) (`/Game/Blueprints/Accessorys/BP_AccessoryBase.Info` _asbp_accessory_base))
  (`/Game/Blueprints/PlayerCharacter/BP_PlayerCharacter.OnGetItem_Event` Interacter)
  (`self.K2_DestroyActor`))

(event `SetItemInfoDefault`)

(fn `UserConstructionScript`
  (`parent.UserConstructionScript`))