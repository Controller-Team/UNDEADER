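; BP_WeaponItem is an interactable weapon pickup that carries its weapon in the WeaponChild child actor component.
; On Interact, it casts the child actor to BP_MasterWeapon, passes that instance to the interacter's ChangeSlotWeapon, then destroys itself.
; If the cast fails, nothing happens; BeginPlay, overlap and Tick are unused, and the construction script only calls its parent.
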(event `self.Interact`
  (params (Interacter :type "/Game/Blueprints/PlayerCharacter/BP_PlayerCharacter Object Reference"))
  (bind _asbp_master_weapon (cast `/Game/Blueprints/Weapons/BP_MasterWeapon` (`ChildActorComponent.ChildActor` (`self.WeaponChild`))))
  (`/Game/Blueprints/PlayerCharacter/BP_PlayerCharacter.ChangeSlotWeapon` Interacter _asbp_master_weapon)
  (`self.K2_DestroyActor`))

(fn `UserConstructionScript`
  (`parent.UserConstructionScript`))