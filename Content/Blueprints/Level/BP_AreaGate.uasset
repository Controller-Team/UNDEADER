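; BP_AreaGate is a level gate that composes an escape area, a milestone and a door as child actors.
; On BeginPlay it casts and caches references to the three child actors.
; InitGate passes the next area type to the milestone and switches the escape area off.
; ActiveGate switches the escape area on and opens the door.
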(event `self.ReceiveBeginPlay`
  (bind _asbp_escape_area (cast `/Game/Blueprints/Level/BP_EscapeArea` (`ChildActorComponent.ChildActor` (`self.BP_EscapeArea`))))
  (set `self.As BP Escape Area` _asbp_escape_area)
  (bind _asbp_mile_stone (cast `/Game/Blueprints/Level/BP_MileStone` (`ChildActorComponent.ChildActor` (`self.BP_MileStone`))))
  (set `self.As BP Mile Stone` _asbp_mile_stone)
  (bind _asbp_door (cast `/Game/Blueprints/Level/BP_Door` (`ChildActorComponent.ChildActor` (`self.BP_Door`))))
  (set `self.As BP Door` _asbp_door))

(event `InitGate`
  (params (`next area type` :type "/Game/Blueprints/Level/AreaType Enum" :default "NewEnumerator0"))
  (`/Game/Blueprints/Level/BP_MileStone.InitMileStone` (`self.As BP Mile Stone`) `next area type`)
  (`/Game/Blueprints/Level/BP_EscapeArea.ToggleEscapeArea` (`self.As BP Escape Area`) false))

(event `ActiveGate`
  (`/Game/Blueprints/Level/BP_EscapeArea.ToggleEscapeArea` (`self.As BP Escape Area`) true)
  (`/Game/Blueprints/Level/BP_Door.OpenDoor` (`self.As BP Door`)))

(fn `UserConstructionScript`)