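; Double door actor that swings its two leaves open and switches on a spotlight when the OpenDoor event runs.
; BeginPlay caches each leaf's relative location, and a timeline's Door track drives their yaw in opposite directions.
; The spotlight reveal hangs off the timeline's Update through a half-second Delay, so it can fire repeatedly during playback.
; No closing logic is present.
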(event `self.ReceiveBeginPlay`
  (set `self.startVecL` (`SceneComponent.RelativeLocation` (`self.DoorL1`)))
  (set `self.startVecR` (`SceneComponent.RelativeLocation` (`self.DoorR`))))

(event `OpenDoor`
  (bind (_direction _door) (`Timeline|타임라인`)
    (:`Update`
      (bind _returnvalue (`KismetMathLibrary.MakeRotator` 0.0 0.0 _door))
      (`SceneComponent.K2_SetRelativeLocationAndRotation` (`self.DoorL1`) (`self.startVecL`) (* _returnvalue -1.0) false false)
      (`SceneComponent.K2_SetRelativeLocationAndRotation` (`self.DoorR`) (`self.startVecR`) _returnvalue false false)
      (`KismetSystemLibrary.Delay` 0.5)
      (`SceneComponent.SetVisibility` (`self.SpotLight`) true false))))

(fn `UserConstructionScript`)