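; BP_EscapeArea is a level exit trigger that sends the player to the next area.
; When the player pawn overlaps its Plane, it calls ToNextArea on the LevelManager held by BP_ThirdPersonGameMode.
; ToggleEscapeArea switches the exit on or off by setting both the actor's visibility and the Plane's collision.
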(event `self.Plane.OnComponentBeginOverlap`
  (params (OverlappedComponent :type "PrimitiveComponent Object Reference") (OtherActor :type "Actor Object Reference") (OtherComp :type "PrimitiveComponent Object Reference") (OtherBodyIndex :type Integer) (bFromSweep :type Boolean) (SweepResult :type "HitResult Structure (by ref)"))
  (if (== OtherActor (`GameplayStatics.GetPlayerPawn` 0))
    (bind _asbp_third_person_game_mode (cast `/Game/Blueprints/BP_ThirdPersonGameMode` (`GameplayStatics.GetGameMode`)))
    (`/Game/Blueprints/Level/BP_LevelManager.ToNextArea` (`/Game/Blueprints/BP_ThirdPersonGameMode.LevelManager` _asbp_third_person_game_mode) "NewEnumerator0")))

(event `ToggleEscapeArea`
  (params (toggle :type Boolean))
  (bind _plane (`self.Plane`))
  (if toggle
    (`self.SetActorHiddenInGame` false)
    (`PrimitiveComponent.SetCollisionEnabled` _plane "QueryAndPhysics")
    (else
      (`self.SetActorHiddenInGame` true)
      (`PrimitiveComponent.SetCollisionEnabled` _plane "NoCollision"))))

(fn `UserConstructionScript`)