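; Level manager that runs each area's countdown, clearing and travel to the next level.
; Tick updates the HUD timer and, every frame at zero, enables escape areas, kills non-sandbag enemies and rolls a reward.
; The reward roll weights type and rarity by area type, but gold ranges and rarity weights are zero and nothing spawns.
; ToNextArea updates the game instance, saves player data, fades and opens one of three levels by count.
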(event `self.ReceiveBeginPlay`
  (`|ExecutionSequence`
    (:`then_0`
      (bind _asbp_third_person_game_mode (cast `/Game/Blueprints/BP_ThirdPersonGameMode` (`GameplayStatics.GetGameMode`)))
      (set `self.WBP HUD` (`/Game/Blueprints/BP_ThirdPersonGameMode.WBP HUD` _asbp_third_person_game_mode))
      (set `self.WBP Fade` (`/Game/Blueprints/BP_ThirdPersonGameMode.WBP Fade` _asbp_third_person_game_mode))
      (bind _asgi_undeader (cast `/Game/Blueprints/GI_Undeader` (`GameplayStatics.GetGameInstance`))
        (:`then`
          (set `self.As GI Undeader` _asgi_undeader))
        (:`CastFailed`
          (`KismetSystemLibrary.PrintString` "level manager: gi underder cast fail"))))
    (:`then_1`
      (`self.ToggleAllEscapeArea` false)
      (`/Game/Blueprints/WBP/WBP_Fade.Do Fade` (`self.WBP Fade`) "Forward" (`self.FadeSpeed`)))
    (:`then_2`
      (if (`self.IsStartLevel`)
        (set `self.LeftEscapeTime` 0.0)))))

(event `ToggleAllEscapeArea`
  (params (toggle :type Boolean))
  (bind _outactors (`GameplayStatics.GetAllActorsOfClass` "/Game/Blueprints/Level/BP_EscapeArea.BP_EscapeArea_C"))
  (for _array_element _outactors
    (`/Game/Blueprints/Level/BP_EscapeArea.ToggleEscapeArea` _array_element toggle)))

(event `self.ReceiveTick`
  (params (DeltaSeconds :type "Float (single-precision)"))
  (bind _output_get (set `self.LeftEscapeTime` (`KismetMathLibrary.FClamp` (- (`self.LeftEscapeTime`) DeltaSeconds) 0.0 99.0)))
  (bind _returnvalue (`KismetMathLibrary.FTrunc` _output_get))
  (`/Game/Blueprints/WBP/WBP_HUD.SetRemainTime` (`self.WBP HUD`) _returnvalue)
  (if (== _returnvalue 0)
    (`self.ToggleAllEscapeArea` true)
    (`self.KillAllEnemy`)
    (`self.SpawnReward`)))

(event `KillAllEnemy`
  (bind _outactors (`GameplayStatics.GetAllActorsOfClass` "/Game/Blueprints/Enemys/BP_EnemyBase.BP_EnemyBase_C"))
  (for _array_element _outactors
    (cast `/Game/Blueprints/Enemys/BP_EnemySandbag` _array_element ; 테스트용 적은 제외
      (:`CastFailed`
        (`/Game/Blueprints/Enemys/BP_EnemyBase.OnKilled` _array_element false)))))

(event `ToNextArea`
  (params (`next Area type` :type "/Game/Blueprints/Level/AreaType Enum" :default "NewEnumerator0"))
  (bind _as_gi_undeader (`self.As GI Undeader`))
  (bind _currlevel (`/Game/Blueprints/GI_Undeader.Update Area Info` _as_gi_undeader (+ (`/Game/Blueprints/GI_Undeader.Get Curr Level Count` _as_gi_undeader) 1) `next Area type`))
  (`KismetSystemLibrary.PrintString` (`KismetStringLibrary.Concat_StrStr` "move to lvl: " (`KismetStringLibrary.Conv_IntToString` _currlevel)) true true (struct :`R` 1.0 :`G` 0.084749 :`A` 1.0) 99.0)
  (`|ExecutionSequence`
    (:`then_0`
      (`/Game/Blueprints/PlayerCharacter/BP_PlayerCharacter.SaveData` (`/Game/Blueprints/BPFL_etc.GetBP_PlayerCharacter` self)))
    (:`then_1`
      (bind _duration (`/Game/Blueprints/WBP/WBP_Fade.Do Fade` (`self.WBP Fade`) "Reverse" (`self.FadeSpeed`)))
      (`KismetSystemLibrary.Delay` _duration)
      (switch `int` (`/Game/Blueprints/GI_Undeader.Get Curr Level Count` (`self.As GI Undeader`))
        (:`1`
          (`GameplayStatics.OpenLevelBySoftObjectPtr` (`self.Level1`)))
        (:`2`
          (`GameplayStatics.OpenLevelBySoftObjectPtr` (`self.Level2`)))
        (:`3`
          (`GameplayStatics.OpenLevelBySoftObjectPtr` (`self.Level3`)))))))

(event `SpawnReward`
  (bind (_rewardtype _goldamont __itemrarirty) (`self.Get Radom Reward` (`/Game/Blueprints/GI_Undeader.CurrAreaType` (`self.As GI Undeader`)))))

(fn `Get Radom Reward`
  (params (`area type` :type "/Game/Blueprints/Level/AreaType Enum" :default "NewEnumerator0"))
  (returns (rewardType :type "/Game/Blueprints/Level/RewardType Enum") (goldAmont :type Integer) (_itemRarirty :type "/Game/Blueprints/ItemRarity Enum"))
  (locals (`weapon per` :type Integer) (`acc per` :type Integer) (`money per` :type Integer) (_RewardType :type "/Game/Blueprints/Level/RewardType Enum") (`_Area type` :type "/Game/Blueprints/Level/AreaType Enum" :default "NewEnumerator0") (goldmin :type Integer) (goldmax :type Integer) (rand :type Integer) (rarityCm :type Integer) (rarityRare :type Integer) (rarityUq :type Integer) (rarity :type "/Game/Blueprints/ItemRarity Enum"))
  (bind __area_type (`local._Area type`))
  (set `local._Area type` `area type`)
  (set `local.rand` (`KismetMathLibrary.RandomIntegerInRange` 0 100))
  (`|ExecutionSequence`
    (:`then_0`
      (switch `/Game/Blueprints/Level/AreaType` (`local._Area type`)
        (:`NewEnumerator0`
          (set `local.weapon per` 10)
          (set `local.acc per` 20)
          (set `local.money per` 70))
        (:`NewEnumerator1`
          (set `local.weapon per` 10)
          (set `local.acc per` 20)
          (set `local.money per` 70))
        (:`NewEnumerator2`
          (set `local.weapon per` 10)
          (set `local.acc per` 20)
          (set `local.money per` 70)))
      (bind _array_index (`/Game/Blueprints/BPFL_etc.Get Idx by Int Arr` (`|MakeArray` (`local.weapon per`) (`local.acc per`) (`local.money per`))))
      (switch `int` _array_index
        (:`0`
          (set `local._RewardType` "NewEnumerator2"))
        (:`1`
          (set `local._RewardType` "NewEnumerator1"))
        (:`2`
          (set `local._RewardType` "NewEnumerator0"))))
    (:`then_1`
      (switch `/Game/Blueprints/Level/RewardType` (`local._RewardType`)
        (:`NewEnumerator0`
          (switch `/Game/Blueprints/Level/AreaType` __area_type
            (:`NewEnumerator0`
              (set `local.goldmin` 0)
              (set `local.goldmax` 0))
            (:`NewEnumerator1`
              (set `local.goldmin` 0)
              (set `local.goldmax` 0))
            (:`NewEnumerator2`
              (set `local.goldmin` 0)
              (set `local.goldmax` 0)))
          (return "NewEnumerator0" (`KismetMathLibrary.RandomIntegerInRange` (`local.goldmin`) (`local.goldmax`)) "NewEnumerator4"))
        (:`NewEnumerator1`
          (switch `/Game/Blueprints/Level/AreaType` __area_type
            (:`NewEnumerator0`
              (set `local.rarityCm` 0)
              (set `local.rarityRare` 0)
              (set `local.rarityUq` 0))
            (:`NewEnumerator1`
              (set `local.rarityCm` 0)
              (set `local.rarityRare` 0)
              (set `local.rarityUq` 0))
            (:`NewEnumerator2`
              (set `local.rarityCm` 0)
              (set `local.rarityRare` 0)
              (set `local.rarityUq` 0)))
          (set `local._RewardType` "NewEnumerator1"))
        (:`NewEnumerator2`
          (switch `/Game/Blueprints/Level/AreaType` __area_type
            (:`NewEnumerator0`
              (set `local.rarityCm` 0)
              (set `local.rarityRare` 0)
              (set `local.rarityUq` 0))
            (:`NewEnumerator1`
              (set `local.rarityCm` 0)
              (set `local.rarityRare` 0)
              (set `local.rarityUq` 0))
            (:`NewEnumerator2`
              (set `local.rarityCm` 0)
              (set `local.rarityRare` 0)
              (set `local.rarityUq` 0)))
          (set `local._RewardType` "NewEnumerator2")))
      (bind _array_index_2 (`/Game/Blueprints/BPFL_etc.Get Idx by Int Arr` (`|MakeArray` (`local.rarityCm`) (`local.rarityRare`) (`local.rarityUq`))))
      (switch `int` _array_index_2
        (:`0`
          (set `local.rarity` "NewEnumerator0"))
        (:`1`
          (set `local.rarity` "NewEnumerator2"))
        (:`2`
          (set `local.rarity` "NewEnumerator3")))
      (return (`local._RewardType`) 0 (`local.rarity`)))))

(fn `IsStartLevel`
  (returns (ReturnValue :type Boolean))
  (return (== (`/Game/Blueprints/GI_Undeader.Get Curr Level Count` (`self.As GI Undeader`)) 0)))

(fn `UserConstructionScript`)