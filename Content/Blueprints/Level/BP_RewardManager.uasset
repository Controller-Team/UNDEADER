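; BP_RewardManager rolls and spawns random area rewards at the level's BP_RewardSpawnPoint.
; Each zone tier (Common, Danger, Chaos) supplies percentage weights for type and rarity, plus gold range and gear count.
; SpawnReward creates a weapon, accessory or resource (money, gear) item actor and sets its chest by rarity.
; Weapons and accessories are picked randomly from data table rows matching the rolled rarity.
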(event `self.ReceiveBeginPlay`
  (`|ExecutionSequence`
    (:`then_0`
      (bind _asgi_undeader (cast `/Game/Blueprints/GI_Undeader` (`GameplayStatics.GetGameInstance`))
        (:`then`
          (set `self.As GI Undeader` _asgi_undeader))
        (:`CastFailed`
          (`KismetSystemLibrary.PrintString` "level manager: gi underder cast fail"))))
    (:`then_1`
      (bind _returnvalue (`GameplayStatics.GetActorOfClass` "/Game/Blueprints/Level/BP_RewardSpawnPoint.BP_RewardSpawnPoint_C"))
      (set `self.rewardPoint` _returnvalue))))

(fn `Get Radom Item Type`
  (params (weaponPer :type Integer) (accPer :type Integer) (moneyPer :type Integer) (gearPer :type Integer))
  (returns (rewardType :type "/Game/Blueprints/DataStructure/ItemType Enum"))
  (locals (`weapon per` :type Integer) (`acc per` :type Integer) (`money per` :type Integer) (_RewardType :type "/Game/Blueprints/DataStructure/ItemType Enum") (`_Area type` :type "/Game/Blueprints/Level/AreaType Enum" :default "NewEnumerator0") (goldmin :type Integer) (goldmax :type Integer) (rand :type Integer) (rarityCm :type Integer) (rarityRare :type Integer) (rarityUq :type Integer) (rarity :type "/Game/Blueprints/ItemRarity Enum") (`gear Per` :type Integer))
  (bind _array_index (`/Game/Blueprints/BPFL_etc.Get Idx by Int Arr` (`|MakeArray` weaponPer accPer moneyPer gearPer)))
  (switch `int` _array_index
    (:`0`
      (return "NewEnumerator2"))
    (:`1`
      (return "NewEnumerator1"))
    (:`2`
      (return "NewEnumerator0"))
    (:`3`
      (return "NewEnumerator4"))))

(fn `Get Radom Rarity`
  (params (commonPer :type Integer) (rarePer :type Integer) (uniquePer :type Integer))
  (returns (`item rarity` :type "/Game/Blueprints/ItemRarity Enum"))
  (locals (`weapon per` :type Integer) (`acc per` :type Integer) (`money per` :type Integer) (_RewardType :type "/Game/Blueprints/DataStructure/ItemType Enum") (`_Area type` :type "/Game/Blueprints/Level/AreaType Enum" :default "NewEnumerator0") (goldmin :type Integer) (goldmax :type Integer) (rand :type Integer) (rarityCm :type Integer) (rarityRare :type Integer) (rarityUq :type Integer) (rarity :type "/Game/Blueprints/ItemRarity Enum"))
  (bind _array_index (`/Game/Blueprints/BPFL_etc.Get Idx by Int Arr` (`|MakeArray` commonPer rarePer uniquePer)))
  (switch `int` _array_index
    (:`0`
      (return "NewEnumerator0"))
    (:`1`
      (return "NewEnumerator2"))
    (:`2`
      (return "NewEnumerator3"))))

(fn `Get Radom Reward by AreaType`
  (params (`area type` :type "/Game/Blueprints/Level/AreaType Enum" :default "NewEnumerator0"))
  (returns (rewardType :type "/Game/Blueprints/DataStructure/ItemType Enum") (playerResAmont :type Integer) (_itemRarirty :type "/Game/Blueprints/ItemRarity Enum"))
  (locals (`weapon per` :type Integer) (`acc per` :type Integer) (`money per` :type Integer) (`gear per` :type Integer) (_RewardType :type "/Game/Blueprints/DataStructure/ItemType Enum") (`_Area type` :type "/Game/Blueprints/Level/AreaType Enum" :default "NewEnumerator0") (goldmin :type Integer) (goldmax :type Integer) (rand :type Integer) (rarityCm :type Integer) (rarityRare :type Integer) (rarityUq :type Integer) (rarity :type "/Game/Blueprints/ItemRarity Enum") (GearCount :type Integer))
  (bind (_rewardtype _playerresamont _itemrarirty) (`self.Get Random Reward` 30 30 20 20 0 60 40 5000 10000 3))
  (bind (_rewardtype_2 _playerresamont_2 _itemrarirty_2) (`self.Get Random Reward` 20 20 50 10 60 40 0 1000 3000 1))
  (bind (_rewardtype_3 _playerresamont_3 _itemrarirty_3) (`self.Get Random Reward` 20 30 40 10 30 50 20 3000 5000 2))
  (switch `/Game/Blueprints/Level/AreaType` `area type`
    (:`NewEnumerator0`
      (return _rewardtype_2 _playerresamont_2 _itemrarirty_2))
    (:`NewEnumerator1`
      (return _rewardtype_3 _playerresamont_3 _itemrarirty_3))
    (:`NewEnumerator2`
      (return _rewardtype _playerresamont _itemrarirty))))

(fn `Get Random Acc Item`
  (params (`Item Rarirty` :type "/Game/Blueprints/ItemRarity Enum" :default "NewEnumerator4"))
  (returns (OutItem :type "/Game/Blueprints/DataStructure/AccData Structure"))
  (locals (`item rarity` :type "/Game/Blueprints/ItemRarity Enum" :default "NewEnumerator4") (`tmp list` :type "Array of /Game/Blueprints/DataStructure/AccData Structure"))
  (set `local.item rarity` `Item Rarirty`)
  (`|ExecutionSequence`
    (:`then_0`
      (bind _outrownames (`DataTableFunctionLibrary.GetDataTableRowNames` "/Game/Blueprints/DataStructure/AccDataTable.AccDataTable"))
      (for _array_element _outrownames
        (bind _returnvalue (`|GetDataTableRow` "/Game/Blueprints/DataStructure/AccDataTable.AccDataTable" _array_element)
          (:`then`
            (if (`|EnumEquality` (`local.item rarity`) (`.raraity_16_C535C83048DC282424E6E0A83E560794` (break `/Game/Blueprints/DataStructure/AccData` _returnvalue)))
              (`KismetArrayLibrary.Array_AddUnique` (`local.tmp list`) _returnvalue))))))
    (:`then_1`
      (return (`KismetArrayLibrary.Array_Random` (`local.tmp list`))))))

(fn `Get Random Reward`
  (params (`weapon per` :type Integer) (`acc per` :type Integer) (`money per` :type Integer) (`gear per` :type Integer) (rarityCm :type Integer) (rarityRare :type Integer) (rarityUq :type Integer) (goldmin :type Integer) (goldmax :type Integer) (GearCount :type Integer))
  (returns (rewardType :type "/Game/Blueprints/DataStructure/ItemType Enum") (playerResAmont :type Integer) (itemRarirty :type "/Game/Blueprints/ItemRarity Enum"))
  (locals (rand :type Integer) (`m_weapon per` :type Integer) (`m_acc per` :type Integer) (`m_money per` :type Integer) (`m_gear per` :type Integer) (m_RewardType :type "/Game/Blueprints/DataStructure/ItemType Enum") (`m_Area type` :type "/Game/Blueprints/Level/AreaType Enum" :default "NewEnumerator0") (m_goldmin :type Integer) (m_goldmax :type Integer) (m_rarityCm :type Integer) (m_rarityRare :type Integer) (m_rarityUq :type Integer) (m_rarity :type "/Game/Blueprints/ItemRarity Enum") (m_GearCount :type Integer))
  (`|ExecutionSequence`
    (:`then_0`
      (set `local.m_weapon per` `weapon per`)
      (set `local.m_acc per` `acc per`)
      (set `local.m_money per` `money per`)
      (set `local.m_gear per` `gear per`)
      (set `local.m_rarityCm` rarityCm)
      (set `local.m_rarityRare` rarityRare)
      (set `local.m_rarityUq` rarityUq)
      (set `local.m_goldmin` goldmin)
      (set `local.m_goldmax` goldmax)
      (set `local.m_GearCount` GearCount))
    (:`then_1`
      (set `local.rand` (`KismetMathLibrary.RandomIntegerInRange` 0 100))
      (`|ExecutionSequence`
        (:`then_0`
          (bind _rewardtype (`self.Get Radom Item Type` (`local.m_weapon per`) (`local.m_acc per`) (`local.m_money per`) (`local.m_gear per`)))
          (set `local.m_RewardType` _rewardtype)
          (bind _item_rarity (`self.Get Radom Rarity` (`local.m_rarityCm`) (`local.m_rarityRare`) (`local.m_rarityUq`)))
          (set `local.m_rarity` _item_rarity))
        (:`then_1`
          (switch `/Game/Blueprints/DataStructure/ItemType` (`local.m_RewardType`)
            (:`NewEnumerator1`
              _)
            (:`NewEnumerator2`
              _)
            (:`NewEnumerator0`
              (return (`local.m_RewardType`) (* (`KismetMathLibrary.FFloor` (/ (`KismetMathLibrary.RandomIntegerInRange` (`local.m_goldmin`) (`local.m_goldmax`)) 100)) 100) (`local.m_rarity`)))
            (:`NewEnumerator4`
              (return (`local.m_RewardType`) (`local.m_GearCount`) (`local.m_rarity`))))
          (return (`local.m_RewardType`) 0 (`local.m_rarity`)))))))

(fn `Get Random Weapon Item`
  (params (`Item Rarirty` :type "/Game/Blueprints/ItemRarity Enum" :default "NewEnumerator4"))
  (returns (OutItem :type "/Game/Blueprints/DataStructure/WeaponData Structure"))
  (locals (`item rarity` :type "/Game/Blueprints/ItemRarity Enum" :default "NewEnumerator4") (`tmp list` :type "Array of /Game/Blueprints/DataStructure/WeaponData Structure"))
  (set `local.item rarity` `Item Rarirty`)
  (`|ExecutionSequence`
    (:`then_0`
      (bind _outrownames (`DataTableFunctionLibrary.GetDataTableRowNames` "/Game/Blueprints/DataStructure/WeaponDataTable.WeaponDataTable"))
      (for _array_element _outrownames
        (bind _returnvalue (`|GetDataTableRow` "/Game/Blueprints/DataStructure/WeaponDataTable.WeaponDataTable" _array_element)
          (:`then`
            (if (`|EnumEquality` (`local.item rarity`) (`.rarity_17_A7D7C98B4F37A28E94EDB1AB4BE40FA2` (break `/Game/Blueprints/DataStructure/WeaponData` _returnvalue)))
              (`KismetArrayLibrary.Array_AddUnique` (`local.tmp list`) _returnvalue))))))
    (:`then_1`
      (return (`KismetArrayLibrary.Array_Random` (`local.tmp list`))))))

(fn `Spawn Reward`
  (params (rewardType1 :type "/Game/Blueprints/DataStructure/ItemType Enum" :default "NewEnumerator3") (resAmount1 :type Integer) (ItemRarity1 :type "/Game/Blueprints/ItemRarity Enum" :default "NewEnumerator4") (SpawnTransform :type "Transform Structure"))
  (returns (`spawn item` :type "/Game/Blueprints/Interactables/Bp_ItemBase Object Reference"))
  (locals (rewardType :type "/Game/Blueprints/DataStructure/ItemType Enum" :default "NewEnumerator3") (resAmount :type Integer :default 0) (ItemRarity :type "/Game/Blueprints/ItemRarity Enum" :default "NewEnumerator4") (`bp item` :type "/Game/Blueprints/Interactables/Bp_ItemBase Object Reference"))
  (bind _bp_item (`local.bp item`))
  (`|ExecutionSequence`
    (:`then_0`
      (set `local.rewardType` rewardType1)
      (set `local.resAmount` resAmount1)
      (set `local.ItemRarity` ItemRarity1))
    (:`then_1`
      (switch `/Game/Blueprints/DataStructure/ItemType` (`local.rewardType`)
        (:`NewEnumerator3`
          (`KismetSystemLibrary.PrintString` "resManager reward type error"))
        (:`NewEnumerator1`
          (bind _returnvalue (`|SpawnActorFromClass` "/Game/Blueprints/Interactables/BP_AccessoryItem.BP_AccessoryItem_C" SpawnTransform "Undefined" "MultiplyWithRoot" null null))
          (set `local.bp item` _returnvalue)
          (`/Game/Blueprints/Interactables/BP_AccessoryItem.InitAccItem` _returnvalue (`self.Get Random Acc Item` (`local.ItemRarity`)))
          (switch `/Game/Blueprints/ItemRarity` (`local.ItemRarity`) :!label _label
            (:`NewEnumerator4`
              (`KismetSystemLibrary.PrintString` "resManager item rarity error" :!label _label_2))
            (:`NewEnumerator0`
              (`/Game/Blueprints/Interactables/Bp_ItemBase.SelectChest` _bp_item "NewEnumerator2"))
            (:`NewEnumerator1`
              (goto _label_2))
            (:`NewEnumerator2`
              (`/Game/Blueprints/Interactables/Bp_ItemBase.SelectChest` _bp_item "NewEnumerator3"))
            (:`NewEnumerator3`
              (`/Game/Blueprints/Interactables/Bp_ItemBase.SelectChest` _bp_item "NewEnumerator4")))
          (return _bp_item))
        (:`NewEnumerator2`
          (bind _returnvalue_2 (`|SpawnActorFromClass` "/Game/Blueprints/Interactables/BP_WeaponItem.BP_WeaponItem_C" SpawnTransform "Undefined" "MultiplyWithRoot" null null))
          (set `local.bp item` _returnvalue_2)
          (`/Game/Blueprints/Interactables/BP_WeaponItem.InitWeaponItem` _returnvalue_2 (`self.Get Random Weapon Item` (`local.ItemRarity`)))
          (goto _label))
        (:`NewEnumerator0`
          (bind _returnvalue_3 (`|SpawnActorFromClass` "/Game/Blueprints/Interactables/BP_ResItem.BP_ResItem_C" SpawnTransform "Undefined" "MultiplyWithRoot" null null :!label _label_3))
          (set `local.bp item` _returnvalue_3)
          (`/Game/Blueprints/Interactables/BP_ResItem.Init` _returnvalue_3 (`local.resAmount`) (`local.rewardType`))
          (goto _label))
        (:`NewEnumerator4`
          (goto _label_3))))))

(fn `SpawnReward by AreaType`
  (params (`area type` :type "/Game/Blueprints/Level/AreaType Enum" :default "NewEnumerator0"))
  (locals (rewardType :type "/Game/Blueprints/DataStructure/ItemType Enum" :default "NewEnumerator3") (resAmount :type Integer :default 0) (ItemRarity :type "/Game/Blueprints/ItemRarity Enum" :default "NewEnumerator4") (`bp item` :type "/Game/Blueprints/Interactables/Bp_ItemBase Object Reference"))
  (bind (_rewardtype _playerresamont __itemrarirty) (`self.Get Radom Reward by AreaType` `area type`))
  (`self.Spawn Reward` _rewardtype _playerresamont __itemrarirty (`self.GetTransform` (`self.rewardPoint`))))

(fn `UserConstructionScript`)