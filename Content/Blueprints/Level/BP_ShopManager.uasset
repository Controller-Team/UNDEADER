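; BP_ShopManager stocks the in-game shop with random items and handles paid rerolls.
; On BeginPlay it gathers spawn points and has the game mode's reward manager spawn shop items there.
; Spawn-point array index fixes each item's category (weapon, accessory or gear), with weighted rarity and upgrade level randomized around level progress.
; Successful rerolls charge money, replace the stock and raise the next price.
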(event `self.ReceiveBeginPlay`
  (`|ExecutionSequence`
    (:`then_0`
      (bind _outactors (`GameplayStatics.GetAllActorsOfClass` "/Game/Blueprints/Level/BP_ShopItemSpawnPoint.BP_ShopItemSpawnPoint_C"))
      (set `self.spawnPoints` _outactors))
    (:`then_1`
      (set `self.BP Reward Manager` (`/Game/Blueprints/BP_ThirdPersonGameMode.BP_RewardManager` (cast `/Game/Blueprints/BP_ThirdPersonGameMode` (`GameplayStatics.GetGameMode`) :!pure true))))
    (:`then_2`
      (`self.SpawnItems`))))

(event `TryReroll`
  (bind _bsuccces_ (`/Game/Blueprints/PlayerRes/BP_PlayerResManager.Try Adjust Money` (`/Game/Blueprints/BPFL_etc.GetBP_ResManager` self) (* (`self.RerollPrice`) -1)))
  (if _bsuccces_
    (`self.SpawnItems`)
    (set `self.RerollPrice` (+ (`self.RerollPrice`) 1000))))

(fn `GetItemLevelByAreaCount`
  (returns (ReturnValue :type Integer))
  (return (`KismetMathLibrary.Clamp` (- (+ (`KismetMathLibrary.FFloor` (/ (`/Game/Blueprints/GI_Undeader.Get Curr Level Count` (cast `/Game/Blueprints/GI_Undeader` (`GameplayStatics.GetGameInstance`) :!pure true)) 5)) 2) (`KismetMathLibrary.RandomIntegerInRange` 0 2)) 0 99)))

(fn `SpawnItems`
  (locals (itemType :type "/Game/Blueprints/DataStructure/ItemType Enum" :default "NewEnumerator3") (itemRarity :type "/Game/Blueprints/ItemRarity Enum" :default "NewEnumerator4") (`weapon Per` :type Integer :default 0) (`acc Per` :type Integer :default 0) (`gear Per` :type Integer :default 0) (`gear Count` :type Integer :default 1) (`cm Per` :type Integer :default 0) (`rare Per` :type Integer :default 0) (`uq Per` :type Integer :default 0))
  (bind _bp_reward_manager (`self.BP Reward Manager`))
  (bind (_rewardtype _playerresamont _itemrarirty) (`/Game/Blueprints/Level/BP_RewardManager.Get Random Reward` _bp_reward_manager (`local.weapon Per`) (`local.acc Per`) 0 (`local.gear Per`) (`local.cm Per`) (`local.rare Per`) (`local.uq Per`) 0 0 (`local.gear Count`)))
  (`|ExecutionSequence`
    (:`then_0`
      (for _array_element (`self.ShopItemList`)
        (`/Engine/EditorBlueprintResources/StandardMacros.IsValid` _array_element
          (:`Is Valid`
            (`self.K2_DestroyActor` _array_element))))
      (`KismetArrayLibrary.Array_Clear` (`self.ShopItemList`)))
    (:`then_2`
      (for (_array_element_2 _array_index) (`self.spawnPoints`)
        (`|ExecutionSequence`
          (:`then_1`
            (set `local.cm Per` 40)
            (set `local.rare Per` 40)
            (set `local.uq Per` 20)
            (set `local.gear Count` 1))
          (:`then_2`
            (switch `int` _array_index
              (:`0`
                (set `local.weapon Per` 100 :!label _label))
              (:`1`
                (goto _label))
              (:`2`
                (set `local.acc Per` 100 :!label _label_2)
                (set `local.weapon Per` 0))
              (:`3`
                (goto _label_2))
              (:`4`
                (set `local.gear Per` 100)
                (set `local.acc Per` 0))))
          (:`then_3`
            (bind _spawn_item (`/Game/Blueprints/Level/BP_RewardManager.Spawn Reward` _bp_reward_manager _rewardtype _playerresamont _itemrarirty (`self.GetTransform` _array_element_2)))
            (`/Game/Blueprints/Interactables/Bp_ItemBase.TrySetUpgradeLevel` _spawn_item (`self.GetItemLevelByAreaCount`))
            (`/Game/Blueprints/Interactables/Bp_ItemBase.InitShopItem` _spawn_item)
            (`KismetArrayLibrary.Array_Add` (`self.ShopItemList`) _spawn_item)))))))

(fn `UserConstructionScript`)