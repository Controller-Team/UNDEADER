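; Player character for a cursor-aimed shooter, with camera-relative movement, sprinting and an afterimage dodge.
; Each tick it applies move input and turns toward the cursor hit point through clamped yaw input.
; Health and stamina components update the HUD, with a hit flash and ragdoll death.
; Pistol and rifle child actors handle equip, semi/auto fire and reload, gated by state checks; slide, jump, melee and aim-zoom graphs are disconnected.
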(event OnInitEventDispatcher(HealthSystem)
  ;[1 1 1] InitSystem
  (CallFunction|UpdateHealthUI))

(event OnAdjustHealthEventDispatcher(HealthSystem)
  ;[1 1 1] InitSystem
  (CallFunction|UpdateHealthUI)
  (CallFunction|HitEffect))

(event OnDeadEventDispatcher(HealthSystem)
  (bind _mesh (Variables|Character|GetMesh))
  ;[1 1 1] InitSystem
  (Collision|SetCollisionEnabled _mesh "PhysicsOnly")
  (Physics|SetSimulatePhysics _mesh true)
  (Components|Activation|SetActive (Variables|Collision|GetCapsuleComponent) false false)
  (Collision|SetCollisionEnabled (Variables|Collision|GetCapsuleComponent) "NoCollision"))

(event Custom|SpwanAfterImage
  ;[1 1 1] Dodge
  (Niagara|SpawnSystemAttached "/Game/VFX/NS_AfterimageSystem_Single.NS_AfterimageSystem_Single" (Variables|Character|GetMesh) "None" "0, 0, 0" "0, 0, 0" "KeepRelativeOffset" false))

(event Custom|UpdateHealthUI
  ;[1 1 1] InitSystem
  (Default|SetHpBar (Variables|Default|GetWBP%20HUD) (Default|GetPercent (Variables|Default|GetHealthSystem))))

(event Custom|MoveCharacter
  ;[1 1 1] Move
  (Pawn|Input|AddMovementInput (Variables|Movement|Getmove%20vector) 1.0 false))

(event Custom|InitStaminaSystem
  ;[1 1 1] InitSystem
  (Utilities|FlowControl|Sequence
    (:then_0
      (Default|InitStamina (Variables|Default|GetStaminaSystem) 4)
      (CallFunction|UpdateStaminaUI))
    (:then_1
      (EventDispatchers|BindEventtoAdjustStaminaED (Variables|Default|GetStaminaSystem) (delegate Custom|UpdateStaminaUI)))))

(event Custom|UpdateStaminaUI
  ;[1 1 1] InitSystem
  (Default|SetStamina (Variables|Default|GetWBP%20HUD) (Default|GetCurrStamina (Variables|Default|GetStaminaSystem))))

(event Custom|CellingTrace
  (bind _returnvalue (Transformation|GetActorLocation))
  (bind _returnvalue_2 (+ _returnvalue "0,0,70.000000"))
  ;[1 1 1] obsoleted
  ;;[1 1 1] Slide
  (bind _returnvalue_3 (Collision|CapsuleTraceByChannel _returnvalue_2 _returnvalue_2 1e+01 5e+01 "TraceTypeQuery1" false (Utilities|Array|MakeArray 0) "None"))
  (if _returnvalue_3
    _))

(event Custom|HitEffect
  (bind _mesh (Variables|Character|GetMesh))
  (Rendering|Material|SetOverlayMaterial _mesh "/Game/Overlay/M_Overlay.M_Overlay" :!class /Script/Engine.MeshComponent)
  (Utilities|FlowControl|Delay 0.15)
  (Rendering|Material|SetOverlayMaterial _mesh 0 :!class /Script/Engine.MeshComponent))

(event Custom|Stop_Sprint
  ;[1 1 1] Sprint
  (Variables|Movement|SetIsSprint false)
  (Variables|/Script/Engine.CharacterMovementComponent|SetMaxWalkSpeed (Variables|Character|GetCharacterMovement) 3e+02))

(event Custom|Start_Sprint
  ;[1 1 1] Sprint
  (Variables|Movement|SetIsSprint true)
  (Variables|/Script/Engine.CharacterMovementComponent|SetMaxWalkSpeed (Variables|Character|GetCharacterMovement) 6e+02))

(event Custom|InitHealthSystem
  ;[1 1 1] InitSystem
  (Default|InitHealthSystem (Variables|Default|GetHealthSystem) 100))

(event Custom|StartDodge
  ;[1 1 1] Dodge
  (if (not (Variables|회피|GetbDodging?))
    (if (!= (Math|Vector|VectorLength (Variables|Movement|Getmove%20vector)) 0.0)
      (Utilities|FlowControl|Sequence
        (:then_0
          (Variables|회피|SetdodgeMove (Variables|Movement|Getmove%20vector))
          (Variables|회피|SetbDodging? true)
          (CallFunction|SpwanAfterImage))
        (:then_1
          (Utilities|FlowControl|Delay (Variables|회피|GetdodgeDuration))
          (CallFunction|EndDodge))
        (:then_2
          (if (Variables|회피|GetbDodging?) :!label _label
            (CallFunction|OnDodge)
            (Utilities|FlowControl|DelayUntilNextTick)
            (goto _label)))))))

(event Custom|OnEndSilde
  ;[1 1 1] obsoleted
  ;;[1 1 1] Slide
  (CallFunction|LookCursor false))

(event Custom|End%20Dodge
  ;[1 1 1] Dodge
  (Variables|회피|SetbDodging? false)
  (Variables|회피|SetdodgeMove "0, 0, 0"))

(event Custom|OnDodge
  ;[1 1 1] Dodge
  (Transformation|AddActorWorldOffset (* (Variables|회피|GetdodgePower) (Variables|회피|GetdodgeMove)) true)
  (Utilities|FlowControl|Delay (Variables|회피|GetAfterImageDelay))
  (CallFunction|SpwanAfterImage))

(event Input|EnhancedActionEvents|EnhancedInputActionIA_Jump
  (params (ActionValue :type Boolean) (ElapsedSeconds :type Float%20%28double-precision%29) (TriggeredSeconds :type Float%20%28double-precision%29) (InputAction :type Input%20Action%20Object%20Reference :default "/Game/Input/Actions/IA_Jump.IA_Jump"))
  ;[1 1 1] obsoleted
)

(event Input|EnhancedActionEvents|EnhancedInputActionIA_Move
  (params (ActionValue :type Vector%202D%20Structure) (ElapsedSeconds :type Float%20%28double-precision%29) (TriggeredSeconds :type Float%20%28double-precision%29) (InputAction :type Input%20Action%20Object%20Reference :default "/Game/Input/Actions/IA_Move.IA_Move"))
  ;[1 1 1] Move
  (:Triggered
    (Variables|Movement|SetAction%20Value%20X (.x ActionValue))
    (Variables|Movement|SetAction%20Value%20Y (* (.y ActionValue) -1.0))
    (Utilities|CanMove
      (:True
        (Variables|Movement|Setmove%20vector (Math|Vector|Normalize (Math|Vector|GetRightVector (Math|Rotator|CombineRotators (Math|Rotator|FindLookatRotation (Math|Vector|MakeVector 0.0 0.0 0.0) (Math|Vector|MakeVector (Variables|Movement|GetAction%20Value%20X) (Variables|Movement|GetAction%20Value%20Y) 0.0)) (Math|Rotator|MakeRotator 0.0 0.0 (.yaw (Transformation|GetWorldRotation (Variables|Camera|GetCameraBoom)))))))))
      (:False
        (Variables|Movement|Setmove%20vector "0, 0, 0" :!label _label))))
  (:Canceled
    (goto _label))
  (:Completed
    (goto _label)))

(event Input|EnhancedActionEvents|EnhancedInputActionIA_Slide
  (params (ActionValue :type Boolean) (ElapsedSeconds :type Float%20%28double-precision%29) (TriggeredSeconds :type Float%20%28double-precision%29) (InputAction :type Input%20Action%20Object%20Reference :default "/Game/Input/Actions/IA_Slide.IA_Slide"))
  ;[1 1 1] obsoleted
  ;;[1 1 1] Slide
)

(event Input|EnhancedActionEvents|EnhancedInputActionIA_Sprint
  (params (ActionValue :type Vector%202D%20Structure) (ElapsedSeconds :type Float%20%28double-precision%29) (TriggeredSeconds :type Float%20%28double-precision%29) (InputAction :type Input%20Action%20Object%20Reference :default "/Game/Input/Actions/IA_Sprint.IA_Sprint"))
  ;[1 1 1] Sprint
  (:Triggered
    (if (not (AI|Components|NavMovement|IsCrouching (Variables|Character|GetCharacterMovement)))
      (CallFunction|StartSprint)))
  (:Completed
    (CallFunction|StopSprint)))

(event Input|EnhancedActionEvents|EnhancedInputActionIA_Dodge
  (params (ActionValue :type Boolean) (ElapsedSeconds :type Float%20%28double-precision%29) (TriggeredSeconds :type Float%20%28double-precision%29) (InputAction :type Input%20Action%20Object%20Reference :default "/Game/Input/Actions/IA_Dodge.IA_Dodge"))
  ;[1 1 1] Dodge
  (:Started
    (bind _bfail_ (Default|UseStamina (Variables|Default|GetStaminaSystem) 1))
    (if (not _bfail_)
      (CallFunction|StartDodge))))

(event Input|EnhancedActionEvents|EnhancedInputActionIA_CameraRotate
  (params (ActionValue :type Float%20%28double-precision%29) (ElapsedSeconds :type Float%20%28double-precision%29) (TriggeredSeconds :type Float%20%28double-precision%29) (InputAction :type Input%20Action%20Object%20Reference :default "/Game/Input/Actions/IA_CameraRotate.IA_CameraRotate"))
  (:Triggered
    (Transformation|AddWorldRotation (Variables|Camera|GetCameraBoom) (Math|Rotator|MakeRotator 0.0 0.0 ActionValue) false false)))

(event EventTick
  (params (DeltaSeconds :type Float%20%28single-precision%29))
  (Utilities|CanMove
    (:True
      (Utilities|FlowControl|Sequence
        (:then_0
          (CallFunction|LookCursor false))
        (:then_1
          (CallFunction|MoveCharacter))))))

(event EventBeginPlay
  (Utilities|FlowControl|Sequence
    (:then_1
      (bind _asbp_third_person_game_mode (Utilities|Casting|CastToBP_ThirdPersonGameMode (Game|GetGameMode)))
      (bind _output_get (Variables|Default|SetAs%20BP%20Third%20Person%20Game%20Mode _asbp_third_person_game_mode))
      (Variables|Default|SetWBP%20HUD (Variables|/Game/Blueprints/BP_ThirdPersonGameMode.BP_ThirdPersonGameMode_C|GetWBP%20HUD _output_get)))
    (:then_2
      (CallFunction|InitAmmoUI)
      (CallFunction|InitHealthSystem)
      (CallFunction|InitStaminaSystem))))

(event EventOnLanded
  (params (Hit :type Hit%20Result%20Structure%20%28by%20ref%29))
  ;[1 1 1] obsoleted
  (CallFunction|ImpactonLand))

(event Input|KeyboardEvents|DebugKeyK
  (params (Key :type Key%20Structure :default "None") (ActionValue :type Input%20Action%20Value%20Structure))
  ;[1 1 1] Test Code
  (:Pressed
    (Default|AdjustHealth (Variables|Default|GetHealthSystem) -10)))

(event Custom|SetCurrWeapon
  (params (weaponType :type Equipt_State%20Enum :default "NewEnumerator4"))
  ;[1 1 1] Weapon Equipt
  (Variables|Weapon|SetEquipt_State weaponType) ; 해당 변수에 대한 SET은\n여기에서만 이루어지게 할 것.
)

(event Custom|ToggleWeaponEquipt
  (params (Selection :type Equipt_State%20Enum :default "NewEnumerator4") (bEquipt? :type Boolean) (bSkipAnimation? :type Boolean))
  ;[1 1 1] Weapon Equipt
  (Utilities|FlowControl|Sequence
    (:then_0
      (switch Utilities|FlowControl|Switch|SwitchonEquipt_State Selection
        (:NewEnumerator5
          (if bEquipt?
            (Variables|Default|SetEquipt%20Montage "/Game/ThirdPerson/Animation/Weapons/Pistol/Montages/MM_Pistol_Equip2.MM_Pistol_Equip2")
            (Variables|Weapon|SetAttach%20Socket%20Name "Pistol_Socket")
            (else
              (Variables|Default|SetEquipt%20Montage "/Game/ThirdPerson/Animation/Weapons/Actions/MM_Generic_Unequip.MM_Generic_Unequip")
              (Variables|Weapon|SetAttach%20Socket%20Name "PistolHost_Socket"))))
        (:NewEnumerator6
          (if bEquipt?
            (Variables|Default|SetEquipt%20Montage "/Game/ThirdPerson/Animation/Weapons/Rifle/Montages/MM_Rifle_Equip1.MM_Rifle_Equip1")
            (Variables|Weapon|SetAttach%20Socket%20Name "Rifle_Socket")
            (else
              (Variables|Default|SetEquipt%20Montage "/Game/ThirdPerson/Animation/Weapons/Actions/MM_Generic_Unequip.MM_Generic_Unequip")
              (Variables|Weapon|SetAttach%20Socket%20Name "RifleHost_Socket"))))))
    (:then_1
      (Default|InitWeapon (Variables|Default|GetAs%20BP%20Master%20Weapon) bEquipt? (Variables|Weapon|GetAttach%20Socket%20Name) Selection))
    (:then_2
      (if (not bSkipAnimation?)
        (Animation|Montage|PlayMontage (Variables|Character|GetMesh) (Variables|Default|GetEquipt%20Montage))))))

(event Custom|ToggleAmmoUI
  (params (bToggle :type Boolean))
  ;[1 1 1] AmmoUI
  (Default|ToggleAmmoUI (Variables|UI|GetAmmoUI) bToggle))

(event Custom|UpdateAmmoUI
  (bind _as_bp_master_weapon (Variables|Default|GetAs%20BP%20Master%20Weapon))
  ;[1 1 1] AmmoUI
  (Default|SetAmmoUI (Variables|UI|GetAmmoUI) (Default|GetCurrAmmo _as_bp_master_weapon) (Variables|/Game/Blueprints/Weapons/BP_MasterWeapon.BP_MasterWeapon_C|GetclipAmmo _as_bp_master_weapon)))

(event Custom|UpdateWeaponData
  (params (Selection :type Equipt_State%20Enum :default "NewEnumerator4"))
  ;[1 1 1] Weapon Equipt
  (Development|PrintString "UpdateWeaponData")
  (switch Utilities|FlowControl|Switch|SwitchonEquipt_State Selection
    (:NewEnumerator4
      (Variables|Default|SetAs%20BP%20Master%20Weapon 0))
    (:NewEnumerator5
      (Variables|Default|SetAs%20BP%20Master%20Weapon (.AsBP%20Master%20Weapon (Utilities|Casting|CastToBP_MasterWeapon (Variables|/Script/Engine.ChildActorComponent|GetChildActor (Variables|Default|GetPistolChild))))))
    (:NewEnumerator6
      (Variables|Default|SetAs%20BP%20Master%20Weapon (.AsBP%20Master%20Weapon (Utilities|Casting|CastToBP_MasterWeapon (Variables|/Script/Engine.ChildActorComponent|GetChildActor (Variables|Default|GetRifleChild))))))))

(event Custom|InitAmmoUI
  ;[1 1 1] AmmoUI
  (Utilities|FlowControl|Sequence
    (:then_0
      (bind _returnvalue (UserInterface|CreateWidget "/Game/ThirdPerson/UI/WBP_Crosshair.WBP_Crosshair_C"))
      (bind _output_get (Variables|UI|SetCrosshairUI _returnvalue))
      (UserInterface|Viewport|AddtoViewport _output_get 0))
    (:then_1
      (bind _returnvalue_2 (UserInterface|CreateWidget "/Game/ThirdPerson/UI/WBP_WeaponAmmo.WBP_WeaponAmmo_C"))
      (bind _output_get_2 (Variables|UI|SetAmmoUI _returnvalue_2))
      (UserInterface|Viewport|AddtoViewport _output_get_2 0)
      (CallFunction|ToggleAmmoUI false))))

(event Custom|FireWeapon
  ;[1 1 1] Fire Event
  (Utilities|IsValid (Variables|Default|GetAs%20BP%20Master%20Weapon)
    (:Is%20Valid
      (Utilities|FlowControl|DoOnce false :!label _label
        (:Completed
          (Utilities|CanUseWeapon
            (:true
              (if (Variables|Input|GetbFireInput?)
                (bind _bfired_ (Default|Fire (Variables|Default|GetAs%20BP%20Master%20Weapon)))
                (if _bfired_
                  (CallFunction|UpdateAmmoUI)
                  (Camera|PlayWorldCameraShake "/Game/Blueprints/Weapons/Fire_CameraShake.Fire_CameraShake_C" (Transformation|GetActorLocation) 0.0 5e+02)
                  (Utilities|FlowControl|Delay (Variables|/Game/Blueprints/Weapons/BP_MasterWeapon.BP_MasterWeapon_C|GetFireInterval (Variables|Default|GetAs%20BP%20Master%20Weapon)))
                  (goto _label Reset)
                  (else
                    (CallFunction|Reload)
                    (goto _label Reset)))))
            (:false
              (goto _label Reset))))))))

(event Custom|Reload
  ;[1 1 1] Reload
  (Variables|Weapon|SetbReloading? true)
  (bind _reloaddelay (Default|Reload (Variables|Default|GetAs%20BP%20Master%20Weapon)))
  (Utilities|FlowControl|Delay _reloaddelay)
  (Variables|Weapon|SetbReloading? false)
  (CallFunction|UpdateAmmoUI))

(event Custom|EquptWeaponToggle
  (bind _input_weapon_type (Variables|Input|GetInput%20Weapon%20Type))
  ;[1 1 1] Weapon Equipt
  (Utilities|FlowControl|Sequence
    (:then_0
      (if (!= (Variables|Weapon|GetEquipt_State) (Math|Conversions|ToInteger(Byte) (Variables|Input|GetInput%20Weapon%20Type))) ; 무기 장비 입력?
        (Utilities|FlowControl|Sequence
          (:then_0
            (if (!= (Variables|Weapon|GetEquipt_State) (Math|Conversions|ToInteger(Byte) (Utilities|Enum|LiteralenumEquipt_State "NewEnumerator4"))) ; 기존 무기 장비중?
              (CallFunction|ToggleWeaponEquipt (Variables|Weapon|GetEquipt_State) false true) ; 기존 장비 애니메이션 없이 해제
            ))
          (:then_1
            (CallFunction|SetCurrWeapon _input_weapon_type)
            (CallFunction|UpdateWeaponData _input_weapon_type)
            (CallFunction|ToggleWeaponEquipt _input_weapon_type true false) ; 새로운 무기 장비
          )
          (:then_2
            (CallFunction|ToggleAmmoUI true)
            (CallFunction|UpdateAmmoUI)))
        (else
          (CallFunction|ToggleWeaponEquipt (Variables|Input|GetInput%20Weapon%20Type) false false)
          (CallFunction|SetCurrWeapon "NewEnumerator4")
          (CallFunction|UpdateWeaponData "NewEnumerator4")
          (CallFunction|ToggleAmmoUI false))))
    (:then_1
      (CallFunction|SetCurrWeapon (Variables|Weapon|GetEquipt_State)))))

(event Input|EnhancedActionEvents|EnhancedInputActionIA_PrimaryWeapons
  (params (ActionValue :type Boolean) (ElapsedSeconds :type Float%20%28double-precision%29) (TriggeredSeconds :type Float%20%28double-precision%29) (InputAction :type Input%20Action%20Object%20Reference :default "/Game/Input/Actions/IA_PrimaryWeapons.IA_PrimaryWeapons"))
  ;[1 1 1] Weapon Equipt
  (:Started
    (Variables|Input|SetInput%20Weapon%20Type "NewEnumerator5")
    (CallFunction|EquptWeaponToggle)))

(event Input|EnhancedActionEvents|EnhancedInputActionIA_SecondaryWeapons
  (params (ActionValue :type Boolean) (ElapsedSeconds :type Float%20%28double-precision%29) (TriggeredSeconds :type Float%20%28double-precision%29) (InputAction :type Input%20Action%20Object%20Reference :default "/Game/Input/Actions/IA_SecondaryWeapons.IA_SecondaryWeapons"))
  ;[1 1 1] Weapon Equipt
  (:Started
    (Variables|Input|SetInput%20Weapon%20Type "NewEnumerator6")
    (CallFunction|EquptWeaponToggle)))

(event Input|EnhancedActionEvents|EnhancedInputActionIA_CameraChange
  (params (ActionValue :type Boolean) (ElapsedSeconds :type Float%20%28double-precision%29) (TriggeredSeconds :type Float%20%28double-precision%29) (InputAction :type Input%20Action%20Object%20Reference :default "/Game/Input/Actions/IA_CameraChange.IA_CameraChange"))
  ;[1 1 1] Obsolated
)

(event Input|EnhancedActionEvents|EnhancedInputActionIA_MeleeAttack
  (params (ActionValue :type Boolean) (ElapsedSeconds :type Float%20%28double-precision%29) (TriggeredSeconds :type Float%20%28double-precision%29) (InputAction :type Input%20Action%20Object%20Reference :default "/Game/Input/Actions/IA_MeleeAttack.IA_MeleeAttack"))
  ;[1 1 1] Obsolated
  ;;[1 1 1] Weapon Melee
)

(event Input|EnhancedActionEvents|EnhancedInputActionIA_Reload
  (params (ActionValue :type Boolean) (ElapsedSeconds :type Float%20%28double-precision%29) (TriggeredSeconds :type Float%20%28double-precision%29) (InputAction :type Input%20Action%20Object%20Reference :default "/Game/Input/Actions/IA_Reload.IA_Reload"))
  ;[1 1 1] Reload
  (:Started
    (Utilities|CanUseWeapon
      (:true
        (CallFunction|Reload)))))

(event Input|EnhancedActionEvents|EnhancedInputActionIA_Fire
  (params (ActionValue :type Boolean) (ElapsedSeconds :type Float%20%28double-precision%29) (TriggeredSeconds :type Float%20%28double-precision%29) (InputAction :type Input%20Action%20Object%20Reference :default "/Game/Input/Actions/IA_Fire.IA_Fire"))
  (bind _as_bp_master_weapon (Variables|Default|GetAs%20BP%20Master%20Weapon))
  (bind _as_bp_master_weapon_2 (Variables|Default|GetAs%20BP%20Master%20Weapon))
  ;[1 1 1] Fire Event
  (:Triggered
    (Utilities|IsValid _as_bp_master_weapon
      (:Is%20Valid
        (switch Utilities|FlowControl|Switch|SwitchonTriggerType (Variables|/Game/Blueprints/Weapons/BP_MasterWeapon.BP_MasterWeapon_C|GettriggerType _as_bp_master_weapon)
          (:NewEnumerator0
            (Variables|Input|SetbFireInput? true :!label _label)
            (CallFunction|FireWeapon))))))
  (:Started
    (Utilities|IsValid _as_bp_master_weapon_2
      (:Is%20Valid
        (switch Utilities|FlowControl|Switch|SwitchonTriggerType (Variables|/Game/Blueprints/Weapons/BP_MasterWeapon.BP_MasterWeapon_C|GettriggerType _as_bp_master_weapon_2)
          (:NewEnumerator1
            (goto _label))))))
  (:Canceled
    (Variables|Input|SetbFireInput? false :!label _label_2))
  (:Completed
    (goto _label_2)))

(event Input|MouseEvents|RightMouseButton
  (params (Key :type Key%20Structure))
  ;[1 1 1] Obsolated
)

(fn ConstructionScript)

(fn ImpactonLand
  (bind _charactermovement (Variables|Character|GetCharacterMovement))
  (bind _velocity (Variables|/Script/Engine.MovementComponent|GetVelocity _charactermovement))
  (bind _returnvalue (Math|Float|Absolute(Float) (.z _velocity)))
  (Utilities|FlowControl|Sequence
    (:then_0
      (if (Math|Float|InRange(Float) _returnvalue 3e+02 9e+02)
        (Variables|Movement|SetLand_State "NewEnumerator4")))
    (:then_1
      (if (Math|Float|InRange(Float) _returnvalue 1e+03 1.2e+03)
        (Variables|Movement|SetLand_State "NewEnumerator5")))
    (:then_2
      (if (> _returnvalue 1.25e+03)
        (Variables|Movement|SetLand_State "NewEnumerator6")))))

(fn LookCursor
  (params (LookMove :type Boolean))
  (bind _returnvalue (Game|GetPlayerController 0))
  (bind _turnspeed (LocalVariables|GetTurnSpeed))
  (bind _hitresult (Game|Player|GetHitResultUnderCursorbyChannel _returnvalue "TraceTypeQuery1" true))
  (bind (_bblockinghit _binitialoverlap _time _distance _location _impactpoint _normal _impactnormal _physmat _hitactor) (Collision|BreakHitResult _hitresult))
  (LocalVariables|Setlook%20move LookMove)
  (Utilities|FlowControl|Sequence
    (:then_0
      ;[1 1 1] 수행예외 처리
      (if (not (.ReturnValue (Class|WidgetLayoutLibrary|GetMousePositionScaledbyDPI (Game|GetPlayerController 0))))
        (return)))
    (:then_1
      ;[1 1 1] 회전 목표 지점 구하기
      (bind _asbp_enemy_base (Utilities|Casting|CastToBP_EnemyBase _hitactor)
        (:then
          (LocalVariables|SetRotationTargetPoint _location))
        (:CastFailed
          (LocalVariables|SetRotationTargetPoint _location))))
    (:then_2
      ;[1 1 1] 목표 회전각 구하기
      (if (and (> (Math|Vector|VectorLength (Variables|Movement|Getmove%20vector)) 0.0) (LocalVariables|Getlook%20move)) ; 커서 방향이 아닌 이동방향으로 회전 && 이동 입력이 있는 경우
        (LocalVariables|SetTargetAngle (.Yaw (Math|Rotator|BreakRotator (Math|Rotator|FindLookatRotation (Math|Vector|MakeVector 0.0 0.0 0.0) (Variables|Movement|Getmove%20vector)))))
        (else
          (LocalVariables|SetTargetAngle (.Yaw (Math|Rotator|BreakRotator (Math|Rotator|FindLookatRotation (Transformation|GetActorLocation) (LocalVariables|GetRotationTargetPoint))))))))
    (:then_3
      ;[1 1 1] 현재 회전각 구하기
      (LocalVariables|SetCurrAngle (.Yaw (Math|Rotator|BreakRotator (Transformation|GetActorRotation)))))
    (:then_4
      ;[1 1 1] 목표 회전값 수정
      (if (> (Math|Float|Absolute(Float) (- (LocalVariables|GetTargetAngle) (LocalVariables|GetCurrAngle))) 1.8e+02) ; 목표와 현재 이루고 있는 각도가 180도 이상? -> 반대로 회전
        (if (>= (LocalVariables|GetTargetAngle) 0.0) ; 목표 각도가 양수?
          (LocalVariables|SetTargetAngle (- -1.8e+02 (- 1.8e+02 (Math|Float|Absolute(Float) (LocalVariables|GetTargetAngle))))) ; 목표 회전값을 음수로 변환(예: 170도 => -190도)
          (else
            (LocalVariables|SetTargetAngle (+ 1.8e+02 (- 1.8e+02 (Math|Float|Absolute(Float) (LocalVariables|GetTargetAngle))))) ; 목표 회전값을 양수로 변환(예: 170도 => -190도)
          ))
        (LocalVariables|SetIntevalAngle (- (LocalVariables|GetTargetAngle) (LocalVariables|GetCurrAngle)))
        (else
          (LocalVariables|SetIntevalAngle (- (LocalVariables|GetTargetAngle) (LocalVariables|GetCurrAngle))))))
    (:then_5
      ;[1 1 1] 회전 적용
      (bind _output_get (LocalVariables|SetMoveAngle (/ (Math|Float|Clamp(Float) (LocalVariables|GetIntevalAngle) (* _turnspeed -1.0) _turnspeed) (Class|PlayerController|GetDeprecatedInputYawScale (Game|GetPlayerController 0)))))
      (Pawn|Input|AddControllerYawInput _output_get) ; 커서를 바라보도록 회전
    )))

(fn GetMuzzleCurrWeapon
  (switch Utilities|FlowControl|Switch|SwitchonEquipt_State (Variables|Weapon|GetEquipt_State)
    (:NewEnumerator4
      (return (Transformation|GetWorldTransform (Variables|Character|GetMesh))))
    (:NewEnumerator5
      (return (Transformation|GetWorldTransform (Variables|/Game/Blueprints/Weapons/BP_MasterWeapon.BP_MasterWeapon_C|GetMuzzle (.AsBP%20Master%20Weapon (Utilities|Casting|CastToBP_MasterWeapon (Variables|/Script/Engine.ChildActorComponent|GetChildActor (Variables|Default|GetPistolChild))))))))
    (:NewEnumerator6
      (return (Transformation|GetWorldTransform (Variables|/Game/Blueprints/Weapons/BP_MasterWeapon.BP_MasterWeapon_C|GetMuzzle (.AsBP%20Master%20Weapon (Utilities|Casting|CastToBP_MasterWeapon (Variables|/Script/Engine.ChildActorComponent|GetChildActor (Variables|Default|GetRifleChild))))))))))