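; Player resource manager that tracks Money and Gear balances and pushes Money to the HUD.
; On BeginPlay it takes the HUD widget from BP_ThirdPersonGameMode and refreshes it.
; Try Adjust functions apply positive amounts directly, but zero or negative amounts only when the balance is at or below that signed amount, returning success.
; Successful changes to either resource call UpdateUI, which displays only Money.
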(event `self.ReceiveBeginPlay`
  (bind _asbp_third_person_game_mode (cast `/Game/Blueprints/BP_ThirdPersonGameMode` (`GameplayStatics.GetGameMode`)))
  (set `self.WBP HUD` (`/Game/Blueprints/BP_ThirdPersonGameMode.WBP HUD` _asbp_third_person_game_mode))
  (`self.UpdateUI`))

(event `UpdateUI`
  (`/Game/Blueprints/WBP/WBP_HUD.SetMoneyUI` (`self.WBP HUD`) (`self.Money`)))

(fn `Try Adjust Gear`
  (params (amount :type Integer))
  (returns (`bSuccces?` :type Boolean))
  (locals (m_amount :type Integer))
  (set `local.m_amount` amount)
  (if (> amount 0)
    _
    (elif (<= (`self.Gear`) (`local.m_amount`))
      _
      (else
        (return false))))
  (set `self.Gear` (+ (`self.Gear`) (`local.m_amount`)))
  (`self.UpdateUI`)
  (return true))

(fn `Try Adjust Money`
  (params (amount :type Integer))
  (returns (`bSuccces?` :type Boolean))
  (locals (m_amount :type Integer))
  (set `local.m_amount` amount)
  (if (> amount 0)
    _
    (elif (<= (`self.Money`) (`local.m_amount`))
      _
      (else
        (return false))))
  (set `self.Money` (+ (`self.Money`) (`local.m_amount`)))
  (`self.UpdateUI`)
  (return true))

(fn `UserConstructionScript`)