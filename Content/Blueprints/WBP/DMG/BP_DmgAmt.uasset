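; BP_DmgAmt is a floating damage number actor that rises from its spawn point and then removes itself.
; On BeginPlay it copies its DmgAmt value into the WBP_DmgAmt widget held by its Widget component.
; The MoveT timeline then lerps the actor a short distance up the world Z axis and destroys it when finished.
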(event `self.ReceiveBeginPlay`
  (bind _aswbp_dmg_amt (cast `/Game/Blueprints/WBP/DMG/WBP_DmgAmt` (`WidgetComponent.GetWidget` (`self.Widget`))))
  (set `/Game/Blueprints/WBP/DMG/WBP_DmgAmt.DmgAmt` (`self.Dmg Amt`) _aswbp_dmg_amt)
  (bind _output_get (set `self.Start Loc` (+ (`self.K2_GetActorLocation`) (0.0 0.0 0.0))))
  (set `self.End Loc` (+ _output_get (0.0 0.0 50.0)))
  (bind (_direction _move_track) (`Timeline|Move T`)
    (:`Update`
      (`self.K2_SetActorLocation` (`KismetMathLibrary.VLerp` (`self.Start Loc`) (`self.End Loc`) _move_track)))
    (:`Finished`
      (`self.K2_DestroyActor`))))

(fn `UserConstructionScript`)