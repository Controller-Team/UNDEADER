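; Base weapon actor for the player's guns, handling hitscan firing, clip ammo, reloading and socket attachment.
; Fire spends a round, traces from the muzzle along the character's forward vector, then spawns tracer, impact, muzzle, sound and montage feedback.
; Enemy hits reduce BP_EnemyBase health using multiplied damage and a random crit roll.
; InitWeapon snaps the player's pistol or rifle child actor to a mesh socket.
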(event `self.ReceiveBeginPlay`
  (bind _asbp_player_character (cast `/Game/Blueprints/PlayerCharacter/BP_PlayerCharacter` (`GameplayStatics.GetPlayerCharacter` 0)))
  (set `self.CharacterRef` _asbp_player_character)
  (set `self.currAmmo` (`self.clipAmmo`)))

(event `InitWeapon`
  (params (bEquiptToggle :type Boolean) (AttachSocketName :type Name) (weaponType :type "/Game/ThirdPerson/DataStructure/Equipt_State Enum" :default "NewEnumerator4"))
  (if bEquiptToggle
    _
    (else
      _))
  (`self.Attach Weapon` AttachSocketName weaponType))

(fn `Attach Weapon`
  (params (SocketName :type Name) (weaponType :type "/Game/ThirdPerson/DataStructure/Equipt_State Enum" :default "NewEnumerator4"))
  (locals (_SocketName :type Name) (TargetChildActor :type "ChildActorComponent Object Reference") (class :type "Actor Class Reference"))
  (bind _characterref (`self.CharacterRef`))
  (bind __socketname (`local._SocketName`))
  (set `local._SocketName` SocketName)
  (switch `/Game/ThirdPerson/DataStructure/Equipt_State` weaponType
    (:`NewEnumerator4`
      (`KismetSystemLibrary.PrintString` "attach weapon : unarmed!"))
    (:`NewEnumerator5`
      (set `local.TargetChildActor` (`/Game/Blueprints/PlayerCharacter/BP_PlayerCharacter.PistolChild` _characterref))
      (`SceneComponent.K2_AttachToComponent` (`local.TargetChildActor`) (`Character.Mesh` (`self.CharacterRef`)) __socketname "SnapToTarget" "SnapToTarget" "SnapToTarget" true :!label _label)
      (`KismetSystemLibrary.PrintString` (`KismetStringLibrary.Concat_StrStr` "eq weapon:" (`|GetEnumeratorNameAsString` weaponType) (`KismetStringLibrary.Conv_NameToString` __socketname))))
    (:`NewEnumerator6`
      (set `local.TargetChildActor` (`/Game/Blueprints/PlayerCharacter/BP_PlayerCharacter.RifleChild` _characterref))
      (goto _label))))

(fn `Bullet_Trace`
  (params (`Socket Location` :type "Vector Structure") (Location :type "Vector Structure") (End :type "Vector Structure"))
  (`|SpawnActorFromClass` "/Game/Weapons/BulletTrace/Bullet_Trace.Bullet_Trace_C" (`KismetMathLibrary.MakeTransform` `Socket Location` (`KismetMathLibrary.FindLookAtRotation` Location End)) "Undefined" "OverrideRootScale" null null))

(fn `CheckCrit`
  (params (`nomal damage` :type "Float (double-precision)") (CritDamageAdd :type "Float (double-precision)") (CritPercentAdd :type "Float (double-precision)"))
  (returns (isCrit :type Boolean) (`out damage` :type "Float (double-precision)"))
  (locals (_nomalDamage :type "Float (double-precision)") (_CritDamAddPercent :type "Float (double-precision)"))
  (set `local._nomalDamage` `nomal damage`)
  (set `local._CritDamAddPercent` CritDamageAdd)
  (if (> (+ CritPercentAdd (`self.CritPercentDefault`)) (`KismetMathLibrary.RandomIntegerInRange` 0 99))
    (return true (`/Game/Blueprints/BPFL_etc.Get Mult Adjusted (increase)` (`local._nomalDamage`) (+ (`self.CritDamAddPercentDefault`) (`local._CritDamAddPercent`))))
    (else
      (return false (`local._nomalDamage`)))))

(fn `Fire`
  (params (DamageMult :type "Float (double-precision)") (CritDamAdd :type "Float (double-precision)") (CritPercentAdd :type "Float (double-precision)"))
  (returns (`bFired?` :type Boolean))
  (locals (_DamageMult :type "Float (double-precision)") (_CritPercentAdd :type "Float (double-precision)") (_CritDamAdd :type "Float (double-precision)"))
  (bind (_bblockinghit _binitialoverlap _time _distance _location _impactpoint _normal _impactnormal _physmat _hitactor _hitcomponent _hitbonename _bonename _hititem _elementindex _faceindex _tracestart _traceend) (`GameplayStatics.BreakHitResult` (`self.Out Hit`)))
  (bind (_bblockinghit_2 _binitialoverlap_2 _time_2 _distance_2 _location_2 _impactpoint_2 _normal_2) (`GameplayStatics.BreakHitResult` (`self.Out Hit`)))
  (bind (_bblockinghit_3 _binitialoverlap_3 _time_3 _distance_3 _location_3 _impactpoint_3 _normal_3 _impactnormal_2 _physmat_2) (`GameplayStatics.BreakHitResult` (`self.Out Hit`)))
  (bind _returnvalue (`SceneComponent.K2_GetComponentLocation` (`self.Muzzle`)))
  (set `local._DamageMult` DamageMult)
  (set `local._CritDamAdd` CritDamAdd)
  (set `local._CritPercentAdd` CritPercentAdd)
  (bind _bfired_ (`self.Fire Check`))
  (if _bfired_
    (`|ExecutionSequence`
      (:`then_0`
        ;[1 1 1] Get Bullet Hit
        (bind _outhit (`KismetSystemLibrary.LineTraceSingle` _returnvalue (+ _returnvalue (* (`self.GetActorForwardVector` (`GameplayStatics.GetPlayerCharacter` 0)) 20000.0)) "TraceTypeQuery4"))
        (set `self.Out Hit` _outhit))
      (:`then_1`
        ;[1 1 1] Bullet Trace
        (`|SpawnActorFromClass` "/Game/Weapons/BulletTrace/Bullet_Trace.Bullet_Trace_C" (`KismetMathLibrary.MakeTransform` _tracestart (`KismetMathLibrary.MakeRotFromX` (- _traceend _tracestart))) "Undefined" "OverrideRootScale" null null))
      (:`then_2`
        ;[1 1 1] Hit FX & Animation
        (`self.Impact VFX` _impactpoint_3 _normal_3 _physmat_2)
        (`self.Play SFX` (`self.FireSound`) "/Game/ThirdPerson/Audio/Concurrency/SCON_Guns_LimitToOwner.SCON_Guns_LimitToOwner")
        (`self.Impact_Decal` "/Game/Weapons/Decal/Impact_Decal.Impact_Decal_C" _location_2 _normal_2 (0.01 0.03 0.03))
        (`self.Muzzle_VFX` (`self.MuzzleNS`) (`self.Muzzle`))
        (`self.PlayMontage` (`self.FireMontage`)))
      (:`then_3`
        (bind _asbp_enemy_base (cast `/Game/Blueprints/Enemys/BP_EnemyBase` (`.HitActor` (`GameplayStatics.BreakHitResult` (`self.Out Hit`)))))
        (`/Game/Blueprints/Components/HealthSystem.AdjustHealth` (`/Game/Blueprints/Enemys/BP_EnemyBase.HealthSystem` _asbp_enemy_base) (`KismetMathLibrary.FTrunc` (`.out damage` (`self.CheckCrit` (`/Game/Blueprints/BPFL_etc.Get Mult Adjusted (increase)` (`KismetMathLibrary.Conv_IntToDouble` (* (`self.Damage`) -1)) (`local._DamageMult`)) (`local._CritDamAdd`) (`local._CritPercentAdd`))))))
      (:`then_4`
        (return true)))
    (else
      ;[1 1 1] Dry On Ammo
      (return false))))

(fn `Fire Check`
  (returns (`bFired?` :type Boolean))
  (locals (WeaponDataRef :type "/Game/ThirdPerson/DataStructure/Weapon_Data Structure"))
  (bind _currammo (`self.currAmmo`))
  (if (>= _currammo 1)
    (set `self.currAmmo` (`KismetMathLibrary.Clamp` (- _currammo 1) 0 (`self.clipAmmo`)))
    (return true)
    (else
      (return false))))

(fn `GetCurrAmmo`
  (returns (currAmmo :type Integer))
  (return (`self.currAmmo`)))

(fn `Impact VFX`
  (params (`Impact Location` :type "Vector Structure") (Normal :type "Vector Structure") (`Physic Mat` :type "PhysicalMaterial Object Reference"))
  (`/Engine/EditorBlueprintResources/StandardMacros.IsValid` `Physic Mat`
    (:`Is Valid`
      (`NiagaraFunctionLibrary.SpawnSystemAtLocation` (select `EPhysicalSurface` (`PhysicalMaterial.SurfaceType` `Physic Mat`) :`SurfaceType_Default` "/Game/Weapons/Effects/Particles/Impacts/NS_Imacts.NS_Imacts" :`SurfaceType1` "/Game/Weapons/Effects/Particles/Impacts/NS_Imacts.NS_Imacts" :!type "NiagaraSystem Object Reference") `Impact Location` (`KismetMathLibrary.Conv_VectorToRotator` Normal)))))

(fn `Impact_Decal`
  (params (Class :type "Actor Class Reference") (Location :type "Vector Structure") (Normal :type "Vector Structure") (Scale :type "Vector Structure"))
  (`|SpawnActorFromClass` Class (`KismetMathLibrary.MakeTransform` Location (`KismetMathLibrary.Conv_VectorToRotator` Normal) Scale) "Undefined" "SelectDefaultAtRuntime" null null))

(fn `Muzzle_VFX`
  (params (SystemTemplate :type "NiagaraSystem Object Reference") (AttachToComponent :type "SceneComponent Object Reference"))
  (`NiagaraFunctionLibrary.SpawnSystemAttached` SystemTemplate AttachToComponent "None" (0.0 0.0 0.0) (struct) "KeepRelativeOffset"))

(fn `Play SFX`
  (params (Sound :type "SoundBase Object Reference") (ConcurrencySettings :type "SoundConcurrency Object Reference"))
  (`GameplayStatics.PlaySound2D` Sound 1.0 1.0 0.0 ConcurrencySettings null false))

(fn `PlayMontage`
  (params (MontageToPlay :type "AnimMontage Object Reference"))
  (returns (Delay :type "Float (single-precision)"))
  (bind _returnvalue (`AnimInstance.Montage_Play` (`SkeletalMeshComponent.GetAnimInstance` (`Character.Mesh` (`self.CharacterRef`))) MontageToPlay 1.0 "Duration" 0.0 true))
  (return _returnvalue))

(fn `Reload`
  (returns (ReloadDelay :type "Float (single-precision)"))
  (bind _delay (`self.PlayMontage` (`self.ReloadMontage`)))
  (`self.Play SFX` (`self.ReloadSound`))
  (set `self.currAmmo` (`self.clipAmmo`))
  (return _delay))

(fn `SetCurrAmmo`
  (params (currAmmo :type Integer))
  (set `self.currAmmo` currAmmo))

(fn `UserConstructionScript`)