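; Double door Blueprint that swings open automatically after a short delay on BeginPlay, marked in a comment as a test trigger.
; A Timeline's Door track drives the relative yaw of the right leaf and the negated yaw of the left leaf, which is also held at a fixed offset.
; The Timeline's Update also feeds a short Delay that switches the SpotLight visible shortly after the motion starts.
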(event `self.ReceiveBeginPlay`
  (`KismetSystemLibrary.Delay` 3.0) ; (Test용) 게임 시작 후 3초 뒤 시작
  (if true
    (bind (_direction _door) (`Timeline|타임라인`)
      (:`Update`
        (bind _returnvalue (`KismetMathLibrary.MakeRotator` 0.0 0.0 _door))
        (`SceneComponent.K2_SetRelativeLocationAndRotation` (`self.DoorL1`) (0.0 290.0 0.0) (* _returnvalue -1.0) false false)
        (`SceneComponent.K2_SetRelativeLocationAndRotation` (`self.DoorR`) (0.0 0.0 0.0) _returnvalue false false)
        (`KismetSystemLibrary.Delay` 0.5)
        (`SceneComponent.SetVisibility` (`self.SpotLight`) true false)))))

(fn `UserConstructionScript`)